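; BP_Scan drives an expanding scan effect by animating the Radius parameter of the M_Scan_Param material parameter collection.
; BeginPlay writes the initial Radius, and Tick calls ScanUpdate, which grows it by AddRadius each frame while IsScan is true, unscaled by delta time.
; At a large fixed limit it clears IsScan and resets Radius to zero; nothing in this Blueprint's graphs sets IsScan true.
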(event EventBeginPlay
  (Rendering|Material|SetScalarParameterValue "/Game/MyGame/Chiga/Material/Post/Scan/M_Scan_Param.M_Scan_Param" "Radius" (Variables|Default|Getradius) :!class /Script/Engine.KismetMaterialLibrary))

(event Collision|EventActorBeginOverlap
  (params (OtherActor :type Actor%20Object%20Reference)))

(event EventTick
  (params (DeltaSeconds :type Float%20%28single-precision%29))
  (CallFunction|ScanUpdate))

(fn ConstructionScript)

(fn ScanUpdate
  (if (Variables|Default|GetisScan)
    (bind _output_get (Variables|Default|Setradius (+ (Variables|Default|Getradius) (LocalVariables|GetaddRadius))))
    (Rendering|Material|SetScalarParameterValue "/Game/MyGame/Chiga/Material/Post/Scan/M_Scan_Param.M_Scan_Param" "Radius" _output_get :!class /Script/Engine.KismetMaterialLibrary)
    (if (>= _output_get 1e+05)
      (Variables|Default|SetisScan false)
      (bind _output_get_2 (Variables|Default|Setradius 0.0))
      (Rendering|Material|SetScalarParameterValue "/Game/MyGame/Chiga/Material/Post/Scan/M_Scan_Param.M_Scan_Param" "Radius" _output_get_2 :!class /Script/Engine.KismetMaterialLibrary))))