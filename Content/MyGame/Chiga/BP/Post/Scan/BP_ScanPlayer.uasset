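; Scan pulse actor that tags NPCs for custom-depth rendering as an expanding sphere reaches them.
; Each tick grows the sphere radius by a fixed, frame-rate-dependent step, clamped to a maximum, and updates overlaps.
; Overlapped BP_NPCBase meshes get custom depth enabled with a stencil value, which this Blueprint never clears.
; BeginPlay stores the start location, which is not read here.
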(event OnComponentBeginOverlap(Sphere)
  (params (OverlappedComponent :type Primitive%20Component%20Object%20Reference) (OtherActor :type Actor%20Object%20Reference) (OtherComp :type Primitive%20Component%20Object%20Reference) (OtherBodyIndex :type Integer) (bFromSweep :type Boolean) (SweepResult :type Hit%20Result%20Structure%20%28by%20ref%29))
  (bind _asbp_npcbase (Utilities|Casting|CastToBP_NPCBase OtherActor))
  (Rendering|SetRenderCustomDepth (Variables|/Script/Engine.Character|GetMesh _asbp_npcbase) true)
  (Rendering|SetCustomDepthStencilValue (Variables|/Script/Engine.Character|GetMesh _asbp_npcbase) 1))

(event EventBeginPlay
  (CallFunction|SetStartPos))

(event Collision|EventActorBeginOverlap
  (params (OtherActor :type Actor%20Object%20Reference)))

(event EventTick
  (params (DeltaSeconds :type Float%20%28single-precision%29))
  (CallFunction|RadiusUpdate))

(fn ConstructionScript)

(fn SetStartPos
  (Variables|Default|SetvectorStart (Transformation|GetActorLocation)))

(fn RadiusUpdate
  (bind _output_get (Variables|Default|SetRadius (+ (Variables|Default|GetRadius) 5e+01)))
  (Components|Sphere|SetSphereRadius (Variables|Default|GetSphere) (Math|Float|Clamp(Float) _output_get 0.0 5e+03) true))