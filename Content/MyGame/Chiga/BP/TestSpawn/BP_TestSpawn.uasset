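; BP_TestSpawn is a test spawner that scatters normal NPCs across a box-sized area.
; Its Construction Script adds MaxNPC child actor components of class BP_NormalNPC and collects them in the Actor array.
; Each gets a random X/Y offset within bounds derived from the Box's world scale, with no height variation.
; The event graph holds only disabled placeholder nodes, so all population happens at construction.
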(event EventBeginPlay)

(event Collision|EventActorBeginOverlap
  (params (OtherActor :type Actor%20Object%20Reference)))

(event EventTick
  (params (DeltaSeconds :type Float%20%28single-precision%29)))

(fn ConstructionScript
  (if (not (== (Variables|Default|GetmaxNPC) 0))
    (LocalVariables|Setlocal_Loction (Transformation|GetWorldLocation (Variables|Default|GetDefaultSceneRoot)))
    (LocalVariables|Setlocal_SpawnSize (Transformation|GetWorldScale (Variables|Default|GetBox)))
    (for _index (range 0 (- (Variables|Default|GetmaxNPC) 1))
      (bind _returnvalue (AddComponent|AddChildActorComponent false))
      (bind _output_get (LocalVariables|SetNewLocalVar_0 _returnvalue))
      (ChildActorComponent|SetChildActorClass _output_get "/Game/MyGame/Toyomura/Blueprints/NPC/BP_NormalNPC.BP_NormalNPC_C")
      (Transformation|AddLocalOffset _output_get (Math|Vector|MakeVector (Math|Random|RandomFloatinRange (* (* (.x (LocalVariables|Getlocal_SpawnSize)) -1.0) 5e+02) (* (.x (LocalVariables|Getlocal_SpawnSize)) 5e+02)) (Math|Random|RandomFloatinRange (* (* (.y (LocalVariables|Getlocal_SpawnSize)) -1.0) 5e+02) (* (.y (LocalVariables|Getlocal_SpawnSize)) 5e+02)) 0.0) false false)
      (Utilities|Array|Add (Variables|Default|GetActor) _returnvalue))))