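; Base hologram actor whose skeletal mesh is visible only while the player pawn is a BP_PlayerDrone, and which expires over time.
; Each Tick updates visibility and adds a fixed 1/60 step to a timer, so lifetime depends on frame rate, destroying the actor at TimeMax.
; Helpers to store a source mesh, randomize TimeMax and invert the visibility rule are defined but not called here.
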(event EventBeginPlay)

(event Collision|EventActorBeginOverlap
  (params (OtherActor :type Actor%20Object%20Reference)))

(event EventTick
  (params (DeltaSeconds :type Float%20%28single-precision%29))
  (CallFunction|ChangeVisible)
  (CallFunction|Update))

(fn ConstructionScript)

(fn ChangeVisible
  (bind _skeletalmesh (Variables|Default|GetSkeletalMesh))
  (Utilities|Casting|CastToBP_PlayerDrone (Game|Player|GetPlayerPawn 0)
    (:then
      (Rendering|SetVisibility _skeletalmesh true false))
    (:CastFailed
      (Rendering|SetVisibility _skeletalmesh false false))))

(fn Init
  (params (mesh :type Character%20Object%20Reference))
  ;[1 1 1] Init
  (Variables|Default|Setcharacter (Variables|/Script/Engine.Character|GetMesh mesh)))

(fn Update
  (bind _output_get (Variables|Default|Settime (+ (Variables|Default|Gettime) 0.016667)))
  (if (>= _output_get (Variables|Default|GettimeMax))
    (Actor|DestroyActor)))

(fn ChangeReVisible
  (bind _skeletalmesh (Variables|Default|GetSkeletalMesh))
  (Utilities|Casting|CastToBP_PlayerDrone (Game|Player|GetPlayerPawn 0)
    (:then
      (Rendering|SetVisibility _skeletalmesh false false))
    (:CastFailed
      (Rendering|SetVisibility _skeletalmesh true false))))

(fn TimeRandomMax
  (Variables|Default|SettimeMax (Math|Random|RandomFloatinRange 1e+01 2e+01)))