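; BP_Exhibition_Child is a child exhibition Blueprint that displays its skeletal mesh as a hologram.
; On BeginPlay it gives every material slot a dynamic instance of M_hologram_Inst and, within the same loop, caches the human player's mesh as Character.
; Each Tick it calls ChangeReVisible, whose logic is defined outside this file.
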(event EventBeginPlay
  (bind _skeletalmesh (Variables|Default|GetSkeletalMesh))
  (for _index (range 0 (Rendering|Material|GetNumMaterials (Variables|Default|GetSkeletalMesh)))
    (bind _returnvalue (Rendering|Material|CreateDynamicMaterialInstance _skeletalmesh _index "/Game/MyGame/Chiga/Material/Hologram/M_hologram_Inst.M_hologram_Inst" "None" :!class /Script/Engine.PrimitiveComponent))
    (Rendering|Material|SetMaterial _skeletalmesh _index _returnvalue)
    (bind _asbp_player_human (Utilities|Casting|CastToBP_PlayerHuman (Game|Player|GetPlayerPawn 0)))
    (Variables|Default|Setcharacter (Variables|/Script/Engine.Character|GetMesh _asbp_player_human))))

(event Collision|EventActorBeginOverlap
  (params (OtherActor :type Actor%20Object%20Reference))
  (|CallParentFunction OtherActor) ; This node is disabled and will not be called.\nDrag off pins to build functionality.
)

(event EventTick
  (params (DeltaSeconds :type Float%20%28single-precision%29))
  (CallFunction|ChangeReVisible))

(fn ConstructionScript
  (|CallParentFunction))