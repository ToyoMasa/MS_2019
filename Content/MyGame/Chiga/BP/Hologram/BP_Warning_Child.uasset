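; BP_Warning_Child is a hologram actor that shows alongside a spawned BP_Warning for a limited time.
; On BeginPlay it gives each skeletal mesh slot a dynamic M_hologram_Inst material, calls TimeRandomMax and spawns the warning at its own transform.
; Tick calls ChangeVisible and adds a fixed 1/60 second to Time, so lifetime depends on frame rate.
; Once Time reaches TimeMax, it destroys itself and the warning.
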(event EventBeginPlay
  (bind _skeletalmesh (Variables|Default|GetSkeletalMesh))
  (|CallParentFunction)
  (for _index (range 0 (Rendering|Material|GetNumMaterials (Variables|Default|GetSkeletalMesh)))
    (bind _returnvalue (Rendering|Material|CreateDynamicMaterialInstance _skeletalmesh _index "/Game/MyGame/Chiga/Material/Hologram/M_hologram_Inst.M_hologram_Inst" "None" :!class /Script/Engine.PrimitiveComponent))
    (Rendering|Material|SetMaterial _skeletalmesh _index _returnvalue))
  (CallFunction|TimeRandomMax)
  (CallFunction|CreateWarning))

(event Collision|EventActorBeginOverlap
  (params (OtherActor :type Actor%20Object%20Reference))
  (|CallParentFunction OtherActor) ; This node is disabled and will not be called.\nDrag off pins to build functionality.
)

(event EventTick
  (params (DeltaSeconds :type Float%20%28single-precision%29))
  (CallFunction|ChangeVisible)
  (bind _output_get (Variables|Default|Settime (+ (Variables|Default|Gettime) 0.016667)))
  (if (>= _output_get (Variables|Default|GettimeMax))
    (Actor|DestroyActor)
    (Actor|DestroyActor (Variables|Default|Getwarinig))))

(fn ConstructionScript
  (|CallParentFunction))

(fn CreateWarning
  (bind _returnvalue (Game|SpawnActorfromClass "/Game/MyGame/Chiga/BP/Warning/BP_warning.BP_Warning_C" (Math|Transform|MakeTransform (Transformation|GetActorLocation) (Transformation|GetActorRotation) "1,1,1") "Undefined" 0 0))
  (Variables|Default|Setwarinig _returnvalue))