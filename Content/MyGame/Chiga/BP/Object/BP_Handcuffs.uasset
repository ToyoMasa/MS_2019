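; BP_Handcuffs is a handcuffs visual actor that animates three static meshes through scale and a material cutoff.
; On BeginPlay, Init gives each mesh its own dynamic instance of M_LightYellow and sets its CutOff to CutOffWidth.
; While IsUpdate is true, Tick calls Play on the Update timeline, whose separate alpha and size tracks drive each mesh's CutOff and uniform world scale.
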(event EventBeginPlay
  (CallFunction|Init))

(event Collision|EventActorBeginOverlap
  (params (OtherActor :type Actor%20Object%20Reference)))

(event EventTick
  (params (DeltaSeconds :type Float%20%28single-precision%29))
  (if (Variables|Default|GetisUpdate)
    (bind (_direction _alpha _size _alpha2 _size2 _alpha3 _size3) (Timeline|Update Play)
      (:Update
        (Rendering|Material|SetScalarParameterValue (Variables|Default|Getmaterial) "CutOff" _alpha :!class /Script/Engine.MaterialInstanceDynamic)
        (Transformation|SetWorldScale3D (Variables|Default|GetStaticMesh) (Math|Conversions|ToVector(Float) _size))
        (Rendering|Material|SetScalarParameterValue (Variables|Default|Getmaterial_0) "CutOff" _alpha2 :!class /Script/Engine.MaterialInstanceDynamic)
        (Transformation|SetWorldScale3D (Variables|Default|GetStaticMesh1) (Math|Conversions|ToVector(Float) _size2))
        (Rendering|Material|SetScalarParameterValue (Variables|Default|Getmaterial_1) "CutOff" _alpha3 :!class /Script/Engine.MaterialInstanceDynamic)
        (Transformation|SetWorldScale3D (Variables|Default|GetStaticMesh2) (Math|Conversions|ToVector(Float) _size3))))))

(fn ConstructionScript)

(fn Init
  (bind _staticmesh (Variables|Default|GetStaticMesh))
  (bind _staticmesh1 (Variables|Default|GetStaticMesh1))
  (bind _staticmesh2 (Variables|Default|GetStaticMesh2))
  (bind _returnvalue (Rendering|Material|CreateDynamicMaterialInstance _staticmesh 0 "/Game/MyGame/Models/Object/M_LightYellow.M_LightYellow" "None" :!class /Script/Engine.PrimitiveComponent))
  (Rendering|Material|SetMaterial _staticmesh 0 _returnvalue)
  (bind _output_get (Variables|Default|Setmaterial _returnvalue))
  (Rendering|Material|SetScalarParameterValue _output_get "CutOff" (Variables|Default|GetCutOffWidth) :!class /Script/Engine.MaterialInstanceDynamic)
  (bind _returnvalue_2 (Rendering|Material|CreateDynamicMaterialInstance _staticmesh1 0 "/Game/MyGame/Models/Object/M_LightYellow.M_LightYellow" "None" :!class /Script/Engine.PrimitiveComponent))
  (Rendering|Material|SetMaterial _staticmesh1 0 _returnvalue_2)
  (bind _output_get_2 (Variables|Default|Setmaterial_0 _returnvalue_2))
  (Rendering|Material|SetScalarParameterValue _output_get_2 "CutOff" (Variables|Default|GetCutOffWidth) :!class /Script/Engine.MaterialInstanceDynamic)
  (bind _returnvalue_3 (Rendering|Material|CreateDynamicMaterialInstance _staticmesh2 0 "/Game/MyGame/Models/Object/M_LightYellow.M_LightYellow" "None" :!class /Script/Engine.PrimitiveComponent))
  (Rendering|Material|SetMaterial _staticmesh2 0 _returnvalue_3)
  (bind _output_get_3 (Variables|Default|Setmaterial_1 _returnvalue_3))
  (Rendering|Material|SetScalarParameterValue _output_get_3 "CutOff" (Variables|Default|GetCutOffWidth) :!class /Script/Engine.MaterialInstanceDynamic))