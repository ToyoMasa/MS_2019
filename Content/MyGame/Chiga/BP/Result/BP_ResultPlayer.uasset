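; BP_ResultPlayer is an actor that hosts four widget components for a result display: top, top shadow, lower-left and lower-right.
; On BeginPlay it casts each component's widget to its result widget class and calls Init, stopping at the first failed cast.
; Tick runs through a two-second Delay into a DoOnce, which switches the Type enum on the top and shadow widgets a single time.
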(event EventBeginPlay
  (bind _asw_result_top (Utilities|Casting|CastToW_ResultTop (UserInterface|GetUserWidgetObject (Variables|Default|GetTop))))
  (Default|Init _asw_result_top)
  (bind _asw_result_to_shadow (Utilities|Casting|CastToW_ResultToShadow (UserInterface|GetUserWidgetObject (Variables|Default|GetShadow_Top))))
  (Default|Init _asw_result_to_shadow)
  (bind _asw_result_donw_left (Utilities|Casting|CastToW_ResultDonwLeft (UserInterface|GetUserWidgetObject (Variables|Default|GetDonwLeft))))
  (Default|Init _asw_result_donw_left)
  (bind _asw_result_donw_right (Utilities|Casting|CastToW_ResultDonwRight (UserInterface|GetUserWidgetObject (Variables|Default|GetDonwRight))))
  (Default|Init _asw_result_donw_right))

(event Collision|EventActorBeginOverlap
  (params (OtherActor :type Actor%20Object%20Reference)))

(event EventTick
  (params (DeltaSeconds :type Float%20%28single-precision%29))
  (Utilities|FlowControl|Delay 2.0)
  (Utilities|FlowControl|DoOnce false
    (:Completed
      (bind _asw_result_top (Utilities|Casting|CastToW_ResultTop (UserInterface|GetUserWidgetObject (Variables|Default|GetTop))))
      (Variables|/Game/MyGame/Chiga/BP/UI/Result/W_ResultTop.W_ResultTop_C|SetType _asw_result_top "NewEnumerator1")
      (bind _asw_result_to_shadow (Utilities|Casting|CastToW_ResultToShadow (UserInterface|GetUserWidgetObject (Variables|Default|GetShadow_Top))))
      (Variables|/Game/MyGame/Chiga/BP/UI/Result/W_ResultToShadow.W_ResultToShadow_C|SetType _asw_result_to_shadow "NewEnumerator1"))))

(fn ConstructionScript)