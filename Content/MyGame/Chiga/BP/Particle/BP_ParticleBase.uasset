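; BP_ParticleBase is a particle effect actor that follows a target actor and shows only while the player pawn is BP_PlayerDrone.
; Each tick it moves the particle system to AttachActor's location and sets visibility by comparing the pawn's display name.
; During its Start state it scales the root up from zero by a fixed, frame-rate-dependent step, then advances the state.
; A separate Attach function snaps it to AttachActor.
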(event EventBeginPlay)

(event Collision|EventActorBeginOverlap
  (params (OtherActor :type Actor%20Object%20Reference)))

(event EventTick
  (params (DeltaSeconds :type Float%20%28single-precision%29))
  (CallFunction|StateUpdate)
  (CallFunction|PositionUpdate)
  (CallFunction|ChangeShouorHidden))

(fn ConstructionScript)

(fn Attach
  (Transformation|AttachActorToActor (Variables|Default|GetattachActor) "None" "SnapToTarget" "KeepRelative" "KeepRelative" true))

(fn PositionUpdate
  (Transformation|SetWorldLocation (Variables|Default|GetParticleSystem) (Transformation|GetActorLocation (Variables|Default|GetattachActor)) false false))

(fn StateUpdate
  (switch Utilities|FlowControl|Switch|SwitchonE_ParticleState (Variables|Default|Getstate)
    (:NewEnumerator0
      (Transformation|SetWorldScale3D (Variables|Default|GetDefaultSceneRoot) (Math|Vector|Lerp(Vector) "0, 0, 0" "1.000000,1.000000,1.000000" (Variables|Default|GetstateTime)))
      (bind _output_get (Variables|Default|SetstateTime (+ (Variables|Default|GetstateTime) 0.008333)))
      (if (>= _output_get 1.0)
        (Variables|Default|SetstateTime 0.0)
        (Variables|Default|Setstate "NewEnumerator1")))))

(fn ChangeShouorHidden
  (if (Utilities|Enum|Equal(Enum) (Utilities|GetDisplayName (Game|Player|GetPlayerPawn 0)) "BP_PlayerDrone")
    (Rendering|SetActorHiddenInGame false)
    (else
      (Rendering|SetActorHiddenInGame true))))