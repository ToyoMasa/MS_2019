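; Gauge icon particle actor that drives a dynamic instance of M_GageIcon_Inst on its particle system.
; Each Tick, ChangeUpdate sets visibility from IsSearch and either fades in a "What" texture via Step, or fades it out.
; Outside the What state, it consumes IsSearch as a per-frame flag to grow or shrink actor scale.
; Change and return flags ramp distortion-style Amout and SpeedY parameters before resetting them; AttachUpdate is empty.
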(event EventBeginPlay
  (bind _particlesystem (Variables|Default|GetParticleSystem))
  (|CallParentFunction)
  (bind _returnvalue (Rendering|Material|CreateDynamicMaterialInstance _particlesystem 0 "/Game/MyGame/Chiga/Material/Icon/M_GageIcon_Inst.M_GageIcon_Inst" "None" :!class /Script/Engine.PrimitiveComponent))
  (Rendering|Material|SetMaterial _particlesystem 0 _returnvalue)
  (Variables|Default|Setmaterial _returnvalue))

(event Collision|EventActorBeginOverlap
  (params (OtherActor :type Actor%20Object%20Reference))
  (|CallParentFunction OtherActor) ; This node is disabled and will not be called.\nDrag off pins to build functionality.
)

(event EventTick
  (params (DeltaSeconds :type Float%20%28single-precision%29))
  (|CallParentFunction DeltaSeconds)
  (CallFunction|ChangeUpdate))

(fn ConstructionScript
  (|CallParentFunction))

(fn AttachUpdate
  (params (gage :type Float%20%28single-precision%29) (AttachLocation :type Vector)))

(fn ChangeUpdate
  (bind _material (Variables|Default|Getmaterial))
  (bind _material_2 (Variables|Default|Getmaterial))
  (bind _material_3 (Variables|Default|Getmaterial))
  (bind _material_4 (Variables|Default|Getmaterial))
  (bind _material_5 (Variables|Default|Getmaterial))
  (Rendering|SetVisibility (Variables|Default|GetParticleSystem) (Variables|Default|GetisSearch) false)
  (if (Variables|Default|GetisWhat)
    (bind _output_get (Variables|Default|SetStep (Math|Float|Clamp(Float) (+ (Variables|Default|GetStep) (* (Utilities|Time|GetWorldDeltaSeconds) 1.5)))))
    (Rendering|Material|SetScalarParameterValue _material_2 "Step" _output_get :!class /Script/Engine.MaterialInstanceDynamic)
    (Rendering|Material|SetTextureParameterValue _material_2 "What" (select (Variables|Default|GetWhatType) "/Game/MyGame/Chiga/Texture/Icon/what02.what02" "/Game/MyGame/Chiga/Texture/Icon/What.What"))
    (else
      (Utilities|FlowControl|Sequence
        (:then_0
          (bind _output_get_2 (Variables|Default|SetStep (Math|Float|Clamp(Float) (- (Variables|Default|GetStep) (Utilities|Time|GetWorldDeltaSeconds)))))
          (Rendering|Material|SetScalarParameterValue (Variables|Default|Getmaterial) "Step" _output_get_2 :!class /Script/Engine.MaterialInstanceDynamic))
        (:then_1
          (if (Variables|Default|GetisSearch)
            (Variables|Default|SetAlphaTime (+ (Variables|Default|GetAlphaTime) 0.016667))
            (Transformation|SetActorScale3D (Math|Vector|Lerp(Vector) "0, 0, 0" "3.000000,3.000000,3.000000" (Variables|Default|GetAlphaTime)))
            (Variables|Default|SetisSearch false)
            (else
              (Variables|Default|SetAlphaTime (- (Variables|Default|GetAlphaTime) 0.016667))
              (Transformation|SetActorScale3D (Math|Vector|Lerp(Vector) "0, 0, 0" "3.000000,3.000000,3.000000" (Variables|Default|GetAlphaTime)))))
          (Variables|Default|SetAlphaTime (Math|Float|Clamp(Float) (Variables|Default|GetAlphaTime))))
        (:then_2
          (if (Class|KismetMathLibrary|XORBoolean (Variables|Default|GetisChange) (Variables|Default|GetisChangeEnd))
            (Variables|Default|SetSpeed (Math|Float|Clamp(Float) (+ (Variables|Default|GetSpeed) (Utilities|Time|GetWorldDeltaSeconds)) 0.0 5.0))
            (bind _output_get_3 (Variables|Default|SetAmout (Math|Float|Clamp(Float) (+ (Variables|Default|GetAmout) (Utilities|Time|GetWorldDeltaSeconds)))))
            (if (>= _output_get_3 0.5)
              (Variables|Default|SetisChangeEnd true)
              (Rendering|Material|SetScalarParameterValue (Variables|Default|Getmaterial) "Change" 1.0 :!class /Script/Engine.MaterialInstanceDynamic)
              (Rendering|Material|SetScalarParameterValue _material "Amout" 0.0 :!class /Script/Engine.MaterialInstanceDynamic)
              (Rendering|Material|SetScalarParameterValue _material "SpeedY" 0.0 :!class /Script/Engine.MaterialInstanceDynamic)
              (Variables|Default|SetSpeed 0.0)
              (Variables|Default|SetAmout 0.0)
              (else
                (Rendering|Material|SetScalarParameterValue _material_3 "Amout" (Variables|Default|GetAmout) :!class /Script/Engine.MaterialInstanceDynamic)
                (Rendering|Material|SetScalarParameterValue _material_3 "SpeedY" (Variables|Default|GetSpeed) :!class /Script/Engine.MaterialInstanceDynamic)))))
        (:then_3
          (if (and (Variables|Default|GetisChangeEnd) (Variables|Default|GetisReturnChange))
            (Variables|Default|SetSpeed (Math|Float|Clamp(Float) (+ (Variables|Default|GetSpeed) (Utilities|Time|GetWorldDeltaSeconds)) 0.0 5.0))
            (bind _output_get_4 (Variables|Default|SetAmout (Math|Float|Clamp(Float) (+ (Variables|Default|GetAmout) (Utilities|Time|GetWorldDeltaSeconds)))))
            (if (>= _output_get_4 0.5)
              (Variables|Default|SetisReturnChange false)
              (Rendering|Material|SetScalarParameterValue (Variables|Default|Getmaterial) "Change" 1.0 :!class /Script/Engine.MaterialInstanceDynamic)
              (Rendering|Material|SetScalarParameterValue _material_4 "Amout" 0.0 :!class /Script/Engine.MaterialInstanceDynamic)
              (Rendering|Material|SetScalarParameterValue _material_4 "SpeedY" 0.0 :!class /Script/Engine.MaterialInstanceDynamic)
              (Variables|Default|SetSpeed 0.0)
              (Variables|Default|SetAmout 0.0)
              (else
                (Rendering|Material|SetScalarParameterValue _material_5 "Amout" (Variables|Default|GetAmout) :!class /Script/Engine.MaterialInstanceDynamic)
                (Rendering|Material|SetScalarParameterValue _material_5 "SpeedY" (Variables|Default|GetSpeed) :!class /Script/Engine.MaterialInstanceDynamic)))))))))