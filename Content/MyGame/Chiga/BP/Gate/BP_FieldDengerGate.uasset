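; Danger gate actor that lights up warning visuals while a BP_PlayerHuman is inside its trigger box.
; On BeginPlay it centers the sign and text between the side posts, sizes boxes and tape, and creates dynamic materials.
; Tick ramps a shared Value into those materials, faster in than out, and feeds player position to the sign.
; While occupied, a timeline animates the ground warning mark and its event re-snaps it to the player's XY.
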(event OnComponentBeginOverlap(Box)
  (params (OverlappedComponent :type Primitive%20Component%20Object%20Reference) (OtherActor :type Actor%20Object%20Reference) (OtherComp :type Primitive%20Component%20Object%20Reference) (OtherBodyIndex :type Integer) (bFromSweep :type Boolean) (SweepResult :type Hit%20Result%20Structure%20%28by%20ref%29))
  (bind _asbp_player_human (Utilities|Casting|CastToBP_PlayerHuman OtherActor))
  (bind _output_get (Variables|Default|Sethuman _asbp_player_human))
  (Variables|Default|SetisValue true)
  (bind _output_get_2 (Variables|Default|Setposition (Math|Vector|MakeVector (.x (Transformation|GetWorldLocation (Variables|/Script/Engine.Character|GetMesh _output_get))) (.y (Transformation|GetWorldLocation (Variables|/Script/Engine.Character|GetMesh _output_get))) 1.5e+02)))
  (Transformation|SetWorldLocation (Variables|Default|GetWarningMarkMesh) _output_get_2 false false))

(event OnComponentEndOverlap(Box)
  (params (OverlappedComponent :type Primitive%20Component%20Object%20Reference) (OtherActor :type Actor%20Object%20Reference) (OtherComp :type Primitive%20Component%20Object%20Reference) (OtherBodyIndex :type Integer))
  (Utilities|Casting|CastToBP_PlayerHuman OtherActor)
  (Variables|Default|SetisValue false)
  (Variables|Default|Sethuman 0))

(event EventBeginPlay
  (CallFunction|Init))

(event Collision|EventActorBeginOverlap
  (params (OtherActor :type Actor%20Object%20Reference)))

(event EventTick
  (params (DeltaSeconds :type Float%20%28single-precision%29))
  (bind _materialwarningmark (Variables|Default|GetmaterialWarningMark))
  (CallFunction|MaterialUpdate DeltaSeconds)
  (if (Variables|Default|GetisValue)
    (bind (_direction _amout _alpha) (Timeline|Amout Play)
      (:Update
        (Rendering|Material|SetScalarParameterValue _materialwarningmark "Amout" _amout :!class /Script/Engine.MaterialInstanceDynamic)
        (Rendering|Material|SetScalarParameterValue _materialwarningmark "Alpha" _alpha :!class /Script/Engine.MaterialInstanceDynamic))
      (:Event
        (|Mark)))
    (else
      (Timeline|Amout PlayFromStart))))

(fn ConstructionScript)

(fn Init
  (CallFunction|InitPosition)
  (CallFunction|InitMaterial))

(fn InitPosition
  (bind _tapemesh (Variables|Default|GetTapeMesh))
  (bind _box1 (Variables|Default|GetBox1))
  (bind _markmesh (Variables|Default|GetMarkMesh))
  (bind _leftmesh (Variables|Default|GetLeftMesh))
  (bind _rightmesh (Variables|Default|GetRightMesh))
  (bind _box (Variables|Default|GetBox))
  (bind _returnvalue (Transformation|GetWorldScale _tapemesh))
  (bind _returnvalue_2 (Transformation|GetWorldScale _markmesh))
  (bind _returnvalue_3 (Transformation|GetWorldLocation _leftmesh))
  (bind _returnvalue_4 (Transformation|GetWorldLocation _rightmesh))
  (bind _returnvalue_5 (Transformation|GetWorldScale _box))
  (bind _returnvalue_6 (Transformation|GetWorldScale _box))
  (bind _returnvalue_7 (- _returnvalue_4 _returnvalue_3))
  (bind _returnvalue_8 (/ _returnvalue_7 2.0))
  (bind _returnvalue_9 (+ _returnvalue_3 _returnvalue_8))
  (Transformation|SetWorldLocation (Variables|Default|GetMarkMesh) (Math|Vector|MakeVector (.x _returnvalue_9) (.y _returnvalue_9) 8e+02) false false)
  (Transformation|SetWorldLocation (Variables|Default|GetFontMesh) (Math|Vector|MakeVector (.x _returnvalue_9) (.y _returnvalue_9) 9e+02) false false)
  (Transformation|SetWorldScale3D _box (Math|Vector|MakeVector (+ (* (.x _returnvalue_2) 3.0) 4.0) (.y _returnvalue_5) (.z _returnvalue_5)))
  (Transformation|SetWorldScale3D _box1 (Math|Vector|MakeVector (.x _returnvalue_6) (.y (Transformation|GetWorldScale _box1)) (.z _returnvalue_6)))
  (Transformation|SetWorldScale3D _tapemesh (Math|Vector|MakeVector (.x _returnvalue_2) (.y _returnvalue) (.z _returnvalue))))

(fn InitMaterial
  (bind _tapemesh (Variables|Default|GetTapeMesh))
  (bind _warningmarkmesh (Variables|Default|GetWarningMarkMesh))
  (bind _markmesh (Variables|Default|GetMarkMesh))
  (bind _fontmesh (Variables|Default|GetFontMesh))
  (bind _materiallines (Variables|Default|GetmaterialLines))
  (bind _leftmesh (Variables|Default|GetLeftMesh))
  (bind _rightmesh (Variables|Default|GetRightMesh))
  (bind _value (Variables|Default|Getvalue))
  (bind _returnvalue (Rendering|Material|CreateDynamicMaterialInstance _markmesh 0 "/Game/MyGame/Chiga/Material/Gate/M_Mark_Inst.M_Mark_Inst" "None" :!class /Script/Engine.PrimitiveComponent))
  (Rendering|Material|SetMaterial _markmesh 0 _returnvalue)
  (Variables|Default|SetmaterialMark _returnvalue)
  (bind _returnvalue_2 (Rendering|Material|CreateDynamicMaterialInstance _fontmesh 0 "/Game/MyGame/Chiga/Material/Gate/M_Font_Inst.M_Font_Inst" "None" :!class /Script/Engine.PrimitiveComponent))
  (Rendering|Material|SetMaterial _fontmesh 0 _returnvalue_2)
  (Variables|Default|SetmaterialFont _returnvalue_2)
  (bind _returnvalue_3 (Rendering|Material|CreateDynamicMaterialInstance _leftmesh 0 "/Game/MyGame/Chiga/Material/Gate/M_GateLine_Inst.M_GateLine_Inst" "None" :!class /Script/Engine.PrimitiveComponent))
  (Rendering|Material|SetMaterial _leftmesh 0 _returnvalue_3)
  (Utilities|Array|Add _materiallines _returnvalue_3)
  (bind _returnvalue_4 (Rendering|Material|CreateDynamicMaterialInstance _rightmesh 0 "/Game/MyGame/Chiga/Material/Gate/M_GateLine_Inst1.M_GateLine_Inst1" "None" :!class /Script/Engine.PrimitiveComponent))
  (Rendering|Material|SetMaterial _rightmesh 0 _returnvalue_4)
  (Utilities|Array|Add _materiallines _returnvalue_4)
  (Rendering|Material|SetScalarParameterValue (Variables|Default|GetmaterialMark) "Value" _value :!class /Script/Engine.MaterialInstanceDynamic)
  (Rendering|Material|SetScalarParameterValue (Variables|Default|GetmaterialMark) "UV" (Variables|Default|GetUV) :!class /Script/Engine.MaterialInstanceDynamic)
  (Rendering|Material|SetScalarParameterValue (Variables|Default|GetmaterialFont) "Value" _value :!class /Script/Engine.MaterialInstanceDynamic)
  (for _array_element (Variables|Default|GetmaterialLines)
    (Rendering|Material|SetScalarParameterValue _array_element "Value" _value :!class /Script/Engine.MaterialInstanceDynamic))
  (bind _returnvalue_5 (Rendering|Material|CreateDynamicMaterialInstance _tapemesh 0 "/Game/MyGame/Chiga/Material/Gate/M_GateTape_Inst.M_GateTape_Inst" "None" :!class /Script/Engine.PrimitiveComponent))
  (Rendering|Material|SetMaterial _tapemesh 0 _returnvalue_5)
  (bind _output_get (Variables|Default|SetmaterialTape _returnvalue_5))
  (Rendering|Material|SetScalarParameterValue _output_get "Value" 0.0 :!class /Script/Engine.MaterialInstanceDynamic)
  (bind _returnvalue_6 (Rendering|Material|CreateDynamicMaterialInstance _warningmarkmesh 0 "/Game/MyGame/Chiga/Material/Noise/M_Noise2_Inst.M_Noise2_Inst" "None" :!class /Script/Engine.PrimitiveComponent))
  (Rendering|Material|SetMaterial _warningmarkmesh 0 _returnvalue_6)
  (Variables|Default|SetmaterialWarningMark _returnvalue_6))

(fn MaterialUpdate
  (params (Time :type Float%20%28single-precision%29))
  (CallFunction|ValueUpdate Time)
  (Rendering|Material|SetVectorParameterValue (Variables|Default|GetmaterialMark) "Position" (Math|Conversions|ToLinearColor(Vector) (Transformation|GetActorLocation (Game|Player|GetPlayerPawn 0))) :!class /Script/Engine.MaterialInstanceDynamic))

(fn ValueUpdate
  (params (Time :type Float%20%28single-precision%29))
  (if (Variables|Default|GetisValue)
    (Variables|Default|Setvalue (Math|Float|Clamp(Float) (+ (Variables|Default|Getvalue) Time)))
    (else
      (Variables|Default|Setvalue (Math|Float|Clamp(Float) (- (Variables|Default|Getvalue) (/ Time 2.0))))))
  (Rendering|Material|SetScalarParameterValue (Variables|Default|GetmaterialMark) "Value" (Variables|Default|Getvalue) :!class /Script/Engine.MaterialInstanceDynamic)
  (Rendering|Material|SetScalarParameterValue (Variables|Default|GetmaterialFont) "Value" (Variables|Default|Getvalue) :!class /Script/Engine.MaterialInstanceDynamic)
  (Rendering|Material|SetScalarParameterValue (Variables|Default|GetmaterialTape) "Value" (Variables|Default|Getvalue) :!class /Script/Engine.MaterialInstanceDynamic)
  (Rendering|Material|SetScalarParameterValue (Variables|Default|GetmaterialWarningMark) "Value" (Variables|Default|Getvalue) :!class /Script/Engine.MaterialInstanceDynamic)
  (for _array_element (Variables|Default|GetmaterialLines)
    (Rendering|Material|SetScalarParameterValue _array_element "Value" (Variables|Default|Getvalue) :!class /Script/Engine.MaterialInstanceDynamic)))