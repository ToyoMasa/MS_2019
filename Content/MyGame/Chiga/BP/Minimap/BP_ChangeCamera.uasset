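; Scene capture actor in the Minimap folder that external code can align to another actor and camera point.
; On BeginPlay it resets the capture's show-only list to this actor's own components.
; SetTransform moves the root to a given actor's world transform and the SceneCaptureComponent2D to a given scene component's transform.
; RotationUpdate copies only an actor's world rotation onto the root, with no per-tick logic.
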(event EventBeginPlay
  (Rendering|SceneCapture|ClearShowOnlyComponents (Variables|Default|GetSceneCaptureComponent2D))
  (Rendering|SceneCapture|ShowOnlyActorComponents (Variables|Default|GetSceneCaptureComponent2D) self))

(event Collision|EventActorBeginOverlap
  (params (OtherActor :type Actor%20Object%20Reference)))

(event EventTick
  (params (DeltaSeconds :type Float%20%28single-precision%29)))

(fn ConstructionScript)

(fn RotationUpdate
  (params (actor :type Static%20Mesh%20Component%20Object%20Reference))
  (Transformation|SetWorldRotation (Variables|Default|GetDefaultSceneRoot) (Transformation|GetWorldRotation actor) false false))

(fn SetTransform
  (params (actor :type Static%20Mesh%20Component%20Object%20Reference) (scene :type Scene%20Capture%20Component%202D%20Object%20Reference))
  (Transformation|SetWorldTransform (Variables|Default|GetDefaultSceneRoot) (Transformation|GetWorldTransform actor) false false)
  (Transformation|SetWorldTransform (Variables|Default|GetSceneCaptureComponent2D) (Transformation|GetWorldTransform scene) false false))