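; Temporary minimap point marker that shows its spawn location and pins to the minimap border when IsHit is false.
; BeginPlay caches that location and gets or creates the GM_MyGame minimap camera.
; Each tick, Position either keeps the mesh there or intersects the spawn-to-player segment with edges from the nearest camera corner, using a 2D segment test.
; After ten seconds it shrinks over one second and destroys itself.
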(event EventBeginPlay
  (Variables|Default|SetStartVector (Transformation|GetWorldLocation (Variables|Default|GetDefaultSceneRoot)))
  (bind _asgm_my_game (Utilities|Casting|CastToGM_MyGame (Game|GetGameInstance)))
  (if (Utilities|IsValid (Variables|/Game/MyGame/BP/GM_MyGame.GM_MyGame_C|GetminimapCamera _asgm_my_game))
    _
    (else
      (Default|CreateMinimapCamera _asgm_my_game)))
  (Variables|Default|SetminimapCamera (Variables|/Game/MyGame/BP/GM_MyGame.GM_MyGame_C|GetminimapCamera _asgm_my_game)))

(event Collision|EventActorBeginOverlap
  (params (OtherActor :type Actor%20Object%20Reference))
  (|CallParentFunction OtherActor) ; This node is disabled and will not be called.\nDrag off pins to build functionality.
)

(event EventTick
  (params (DeltaSeconds :type Float%20%28single-precision%29))
  (CallFunction|Position)
  (bind _output_get (Variables|Default|Settime (Math|Float|Clamp(Float) (+ DeltaSeconds (Variables|Default|Gettime)) 0.0 1e+01)))
  (if (>= _output_get 1e+01)
    (Variables|Default|SettimeSize (Math|Float|Clamp(Float) (+ (Variables|Default|GettimeSize) DeltaSeconds)))
    (Transformation|SetWorldScale3D (Variables|Default|GetStaticMesh) (Math|Conversions|ToVector(Float) (Math|Float|Lerp (.x (Variables|Default|Getsize)) 0.0 (Math|Float|Clamp(Float) (+ (Variables|Default|GettimeSize) DeltaSeconds)))))
    (if (>= (Variables|Default|GettimeSize) 1.0)
      (Actor|DestroyActor))))

(fn ConstructionScript
  (|CallParentFunction))

(fn Position
  (bind _returnvalue (Game|Player|GetPlayerPawn 0))
  (bind _startvector (Variables|Default|GetStartVector))
  (bind _startvector_2 (Variables|Default|GetStartVector))
  (bind _minimapcamera (Variables|Default|GetminimapCamera))
  (bind _returnvalue_2 (Transformation|GetActorLocation _returnvalue))
  (if (Variables|Default|GetisHit)
    (Transformation|SetWorldLocation (Variables|Default|GetStaticMesh) (Math|Vector|MakeVector (.x _startvector_2) (.y _startvector_2) 5e+02) false false)
    (elif (Utilities|IsValid (Variables|Default|GetminimapCamera))
      (bind _output_get (LocalVariables|SetminimapScene (Utilities|Array|MakeArray (Variables|/Game/MyGame/Chiga/BP/Minimap/BP_MinimapCamera.BP_MinimapCamera_C|GetL_U _minimapcamera) (Variables|/Game/MyGame/Chiga/BP/Minimap/BP_MinimapCamera.BP_MinimapCamera_C|GetL_D _minimapcamera) (Variables|/Game/MyGame/Chiga/BP/Minimap/BP_MinimapCamera.BP_MinimapCamera_C|GetR_U _minimapcamera) (Variables|/Game/MyGame/Chiga/BP/Minimap/BP_MinimapCamera.BP_MinimapCamera_C|GetR_D _minimapcamera))))
      (for (_array_element _array_index) _output_get
        (if (== _array_index 0)
          (Variables|Default|SetLength (Math|Vector|VectorLength (- (Variables|Default|GetStartVector) (Math|Vector|MakeVector (.x (Transformation|GetWorldLocation _array_element)) (.y (Transformation|GetWorldLocation _array_element)) 5e+02))))
          (LocalVariables|Setindex 0)
          (elif (not (== (Math|Float|Min(Float) (Math|Vector|VectorLength (- (Variables|Default|GetStartVector) (Math|Vector|MakeVector (.x (Transformation|GetWorldLocation _array_element)) (.y (Transformation|GetWorldLocation _array_element)) 5e+02))) (Variables|Default|GetLength)) (Variables|Default|GetLength)))
            (Variables|Default|SetLength (Math|Float|Min(Float) (Math|Vector|VectorLength (- (Variables|Default|GetStartVector) (Math|Vector|MakeVector (.x (Transformation|GetWorldLocation _array_element)) (.y (Transformation|GetWorldLocation _array_element)) 5e+02))) (Variables|Default|GetLength)))
            (LocalVariables|Setindex _array_index))))
      (bind _nextpositions (Default|GetCrossPositions (Variables|Default|GetminimapCamera) (Utilities|Array|Get(acopy) (LocalVariables|GetminimapScene) (LocalVariables|Getindex))))
      (bind _array_element_2 (Utilities|Array|ForEachLoopwithBreak _nextpositions)
        (:LoopBody
          (bind (_hit _crossposition) (CallFunction|CrossPosition (Math|Vector|MakeVector (.x (Transformation|GetWorldLocation (Utilities|Array|Get(acopy) (LocalVariables|GetminimapScene) (LocalVariables|Getindex)))) (.y (Transformation|GetWorldLocation (Utilities|Array|Get(acopy) (LocalVariables|GetminimapScene) (LocalVariables|Getindex)))) 1e+02) (Math|Vector|MakeVector (.x (Transformation|GetWorldLocation _array_element_2)) (.y (Transformation|GetWorldLocation _array_element_2)) 1e+02) (Math|Vector|MakeVector (.x _startvector) (.y _startvector) 1e+02) (Math|Vector|MakeVector (.x _returnvalue_2) (.y _returnvalue_2) 1e+02)))
          (if _hit
            (Transformation|SetWorldLocation (Variables|Default|GetStaticMesh) (Math|Vector|MakeVector (.x _crossposition) (.y _crossposition) 5e+02) false false))))
      (else
        (Actor|DestroyActor)))))

(fn Scale
  (if (Variables|Default|GetisHit)
    (bind _output_get (Variables|Default|Setsize "1.000000,1.000000,1.000000"))
    (Transformation|SetWorldScale3D (Variables|Default|GetStaticMesh) _output_get)
    (else
      (bind _output_get_2 (Variables|Default|Setsize "1.500000,1.500000,1.500000"))
      (Transformation|SetWorldScale3D (Variables|Default|GetStaticMesh) _output_get_2))))

(fn CrossPosition
  (params (p1 :type Vector) (p2 :type Vector) (p3 :type Vector) (p4 :type Vector))
  (LocalVariables|Setlocal_p1 p1)
  (LocalVariables|Setlocal_p2 p2)
  (LocalVariables|Setlocal_p3 p3)
  (LocalVariables|Setlocal_p4 p4)
  (if (== (- (* (- (.x (LocalVariables|Getlocal_p2)) (.x (LocalVariables|Getlocal_p1))) (- (.y (LocalVariables|Getlocal_p4)) (.y (LocalVariables|Getlocal_p3)))) (* (- (.y (LocalVariables|Getlocal_p2)) (.y (LocalVariables|Getlocal_p1))) (- (.x (LocalVariables|Getlocal_p4)) (.x (LocalVariables|Getlocal_p3))))) 0.0)
    (return false "0, 0, 0")
    (else
      (LocalVariables|Setlocal_d (- (* (- (.x (LocalVariables|Getlocal_p2)) (.x (LocalVariables|Getlocal_p1))) (- (.y (LocalVariables|Getlocal_p4)) (.y (LocalVariables|Getlocal_p3)))) (* (- (.y (LocalVariables|Getlocal_p2)) (.y (LocalVariables|Getlocal_p1))) (- (.x (LocalVariables|Getlocal_p4)) (.x (LocalVariables|Getlocal_p3))))))
      (LocalVariables|Setlocal_U (/ (- (* (- (.x (LocalVariables|Getlocal_p3)) (.x (LocalVariables|Getlocal_p1))) (- (.y (LocalVariables|Getlocal_p4)) (.y (LocalVariables|Getlocal_p3)))) (* (- (.y (LocalVariables|Getlocal_p3)) (.y (LocalVariables|Getlocal_p1))) (- (.x (LocalVariables|Getlocal_p4)) (.x (LocalVariables|Getlocal_p3))))) (LocalVariables|Getlocal_d)))
      (LocalVariables|Setlocal_V (/ (- (* (- (.x (LocalVariables|Getlocal_p3)) (.x (LocalVariables|Getlocal_p1))) (- (.y (LocalVariables|Getlocal_p2)) (.y (LocalVariables|Getlocal_p1)))) (* (- (.y (LocalVariables|Getlocal_p3)) (.y (LocalVariables|Getlocal_p1))) (- (.x (LocalVariables|Getlocal_p2)) (.x (LocalVariables|Getlocal_p1))))) (LocalVariables|Getlocal_d)))
      (if (or (or (< (LocalVariables|Getlocal_U) 0.0) (> (LocalVariables|Getlocal_U) 1.0)) (or (< (LocalVariables|Getlocal_V) 0.0) (> (LocalVariables|Getlocal_V) 1.0)))
        (return false "0, 0, 0")
        (else
          (return true (Math|Vector|MakeVector (+ (* (- (.x (LocalVariables|Getlocal_p2)) (.x (LocalVariables|Getlocal_p1))) (LocalVariables|Getlocal_U)) (.x (LocalVariables|Getlocal_p1))) (+ (* (- (.y (LocalVariables|Getlocal_p2)) (.y (LocalVariables|Getlocal_p1))) (LocalVariables|Getlocal_U)) (.y (LocalVariables|Getlocal_p1))) 5e+02)))))))