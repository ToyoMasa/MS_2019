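; BP_MinimapCamera is the top-down scene capture camera behind the minimap, creating the minimap and game score widgets at BeginPlay.
; Each tick it follows the player at fixed height Zpos, looking straight down with yaw matched to the player camera.
; Its capture uses a show-only list seeded with BP_MinimapCamera and BP_MinimapUI actors, editable through ShowUI and RemoveShou.
; The player's IsMinimap flag switches the minimap widget's FadeType every tick.
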(event EventBeginPlay
  (bind _asbp_player_human (Utilities|Casting|CastToBP_PlayerHuman (Game|Player|GetPlayerPawn 0)))
  (Variables|Default|Sethuman _asbp_player_human)
  (CallFunction|Show)
  (bind _returnvalue (UserInterface|CreateWidget "/Game/MyGame/Chiga/BP/UI/W_Minimap.W_Minimap_C"))
  (bind _output_get (Variables|Default|SetminimapUI _returnvalue))
  (UserInterface|Viewport|AddtoViewport _output_get 0)
  (bind _returnvalue_2 (UserInterface|CreateWidget "/Game/MyGame/Chiga/BP/UI/W_GameScore.W_GameScore_C"))
  (UserInterface|Viewport|AddtoViewport _returnvalue_2 0))

(event Collision|EventActorBeginOverlap
  (params (OtherActor :type Actor%20Object%20Reference)))

(event EventTick
  (params (DeltaSeconds :type Float%20%28single-precision%29))
  (CallFunction|PlayerPos)
  (CallFunction|Rotate)
  (CallFunction|Change))

(fn ConstructionScript)

(fn PlayerPos
  (bind _returnvalue (Game|GetPlayerCharacter 0))
  (Transformation|SetActorLocation (+ (- (Transformation|GetActorLocation _returnvalue) (Math|Vector|MakeVector 0.0 0.0 (.z (Transformation|GetActorLocation _returnvalue)))) (Math|Vector|MakeVector 0.0 0.0 (Variables|Default|GetZpos))) false false))

(fn Show
  ;[1 1 1] 描画対象
  (bind _outactors (Actor|GetAllActorsOfClass "BP_MinimapCamera_C"))
  (for _array_element _outactors
    (Rendering|SceneCapture|ShowOnlyActorComponents (Variables|Default|GetSceneCaptureComponent2D) _array_element)
    (bind _outactors_2 (Actor|GetAllActorsOfClass "/Game/MyGame/Chiga/BP/Minimap/BP_MinimapUI.BP_MinimapUI_C"))
    (for _array_element_2 _outactors_2
      (Rendering|SceneCapture|ShowOnlyActorComponents (Variables|Default|GetSceneCaptureComponent2D) _array_element_2))))

(fn ShowUI
  (params (SetShow :type Actor%20Object%20Reference))
  (Rendering|SceneCapture|ShowOnlyActorComponents (Variables|Default|GetSceneCaptureComponent2D) SetShow))

(fn RemoveShou
  (params (remove :type Actor%20Object%20Reference))
  (Class|SceneCaptureComponent|RemoveShowOnlyActorComponents (Variables|Default|GetSceneCaptureComponent2D) remove))

(fn Change
  (bind _minimapui (Variables|Default|GetminimapUI))
  (if (Variables|/Game/MyGame/Toyomura/Blueprints/Player/BP_PlayerHuman.BP_PlayerHuman_C|GetisMinimap (Variables|Default|Gethuman))
    (Variables|/Game/MyGame/Chiga/BP/UI/W_Minimap.W_Minimap_C|SetfadeType _minimapui "NewEnumerator1")
    (else
      (Variables|/Game/MyGame/Chiga/BP/UI/W_Minimap.W_Minimap_C|SetfadeType _minimapui "NewEnumerator0"))))

(fn Rotate
  (Transformation|SetActorRotation (Math|Rotator|MakeRotator 0.0 -9e+01 (.yaw (Transformation|GetActorRotation (Game|GetPlayerCameraManager 0))))))