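; BP_warning is a warning marker of four poles, four tapes and a particle system, shown only while player 0's pawn is a BP_PlayerDrone.
; BeginPlay gives each mesh a dynamic pole or tape material instance and stores it in Materials.
; Tick counts Lenght down by one per frame, clamped between zero and an upper limit, feeds it to each material's "Length" parameter, then updates visibility via Change.
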(event EventBeginPlay
  ;[1 1 1] Material設定
  (bind _output_get (Variables|Default|Setmeshs (Utilities|Array|MakeArray (Variables|Default|Get1) (Variables|Default|Get2) (Variables|Default|Get3) (Variables|Default|Get4) (Variables|Default|GetTape1) (Variables|Default|GetTape2) (Variables|Default|GetTape3) (Variables|Default|GetTape4))))
  (for (_array_element _array_index) _output_get
    (if (> _array_index 3)
      (bind _returnvalue (Rendering|Material|CreateDynamicMaterialInstance _array_element 0 "/Game/MyGame/Chiga/Mesh/Warning/M_Tape_Inst.M_Tape_Inst" "None" :!class /Script/Engine.PrimitiveComponent))
      (Rendering|Material|SetMaterial _array_element 0 _returnvalue)
      (Utilities|Array|Add (Variables|Default|Getmaterials) _returnvalue)
      (else
        (bind _returnvalue_2 (Rendering|Material|CreateDynamicMaterialInstance _array_element 0 "/Game/MyGame/Chiga/Mesh/Warning/M_Pole_Inst.M_Pole_Inst" "None" :!class /Script/Engine.PrimitiveComponent))
        (Rendering|Material|SetMaterial _array_element 0 _returnvalue_2)
        (Utilities|Array|Add (Variables|Default|Getmaterials) _returnvalue_2)))))

(event Collision|EventActorBeginOverlap
  (params (OtherActor :type Actor%20Object%20Reference)))

(event EventTick
  (params (DeltaSeconds :type Float%20%28single-precision%29))
  (CallFunction|MaterialUpdate)
  (CallFunction|Change))

(fn ConstructionScript)

(fn Change
  (bind _1 (Variables|Default|Get1))
  (Utilities|Casting|CastToBP_PlayerDrone (Game|Player|GetPlayerPawn 0)
    (:then
      (Rendering|SetVisibility _1 true false))
    (:CastFailed
      (Rendering|SetVisibility _1 false false))))

(fn MaterialUpdate
  (bind _output_get (Variables|Default|SetLenght (Math|Float|Clamp(Float) (- (Variables|Default|GetLenght) 1.0) 0.0 2e+02)))
  (for _array_element (Variables|Default|Getmaterials)
    (Rendering|Material|SetScalarParameterValue _array_element "Length" _output_get :!class /Script/Engine.MaterialInstanceDynamic)))