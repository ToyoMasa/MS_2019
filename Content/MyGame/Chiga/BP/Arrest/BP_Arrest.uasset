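; BP_Arrest is an actor that drives a Niagara effect (EB_Test1) attached to a supplied mesh through CreateArrest.
; Each Tick lowers Position by a fixed, frame-rate-dependent step, clamps it, and writes it to the emitter's position parameter.
; The effect auto-destroys on completion, and the actor destroys itself on Tick once the Niagara reference is invalid.
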(event EventBeginPlay)

(event Collision|EventActorBeginOverlap
  (params (OtherActor :type Actor%20Object%20Reference)))

(event EventTick
  (params (DeltaSeconds :type Float%20%28single-precision%29))
  (CallFunction|NiagaraUpdate)
  (if (not (Utilities|IsValid (Variables|Default|GetNiagara)))
    (Actor|DestroyActor)))

(fn ConstructionScript)

(fn CreateArrest
  (params (mesh :type Skeletal%20Mesh%20Component%20Object%20Reference))
  (bind _returnvalue (Transformation|GetActorTransform))
  (bind _returnvalue_2 (Niagara|SpawnSystemAttached "/Game/MyGame/Chiga/Particle/Arrest/Test/EB_Test1.EB_Test1" mesh "None" (.location _returnvalue) (.rotation _returnvalue) "KeepRelativeOffset" true))
  (Variables|Default|SetNiagara _returnvalue_2))

(fn NiagaraUpdate
  (bind _output_get (Variables|Default|Setposition (Math|Float|Clamp(Float) (- (Variables|Default|Getposition) 0.016667) 0.0 1e+02)))
  (Niagara|SetNiagaraVariable(Float) (Variables|Default|GetNiagara) "Emitter.position" _output_get))