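; Blueprint helper functions that randomize NPC appearance through material textures and accessory meshes.
; Face and body functions each pick one random index to set matching color and "Rafnes" textures, plus a normal map for the body.
; Hair always gets a random mesh, while glasses, hat, AC and two sub slots roll a coin flip and return whether one was applied.
; Glasses use the returned face index to skip listed faces.
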(fn NPCRandomTextureFace
  (params (material :type Material%20Instance%20Dynamic%20Object%20Reference))
  (bind _output_get (LocalVariables|SetRandom (Math|Random|RandomIntegerinRange 0 66)))
  (Rendering|Material|SetTextureParameterValue material "Face_Color" (Utilities|Array|Get(acopy) (LocalVariables|GetBaseTexture) _output_get))
  (Rendering|Material|SetTextureParameterValue material "Face_Rafnes" (Utilities|Array|Get(acopy) (LocalVariables|GetRafnesTexture) _output_get))
  (return _output_get))

(fn NPCRandomTextureBody
  (params (material :type Material%20Instance%20Dynamic%20Object%20Reference))
  (bind _output_get (LocalVariables|SetRandom (Math|Random|RandomIntegerinRange 0 52)))
  (Rendering|Material|SetTextureParameterValue material "Body_Color" (Utilities|Array|Get(acopy) (LocalVariables|GetBaseTexture) _output_get))
  (Rendering|Material|SetTextureParameterValue material "Body_Rafnes" (Utilities|Array|Get(acopy) (LocalVariables|GetRafnesTexture) _output_get))
  (Rendering|Material|SetTextureParameterValue material "Body_Normal" (Utilities|Array|Get(acopy) (LocalVariables|GetNormalTexture) _output_get)))

(fn NPCRandomHair
  (params (hair :type Static%20Mesh%20Component%20Object%20Reference))
  (Components|StaticMesh|SetStaticMesh hair (Utilities|Array|Get(acopy) (LocalVariables|Getlocal_Mesh) (Math|Random|RandomIntegerinRange 0 3))))

(fn NPCRandomGlass
  (params (faceRandom :type Integer) (mesh :type Static%20Mesh%20Component%20Object%20Reference))
  (if (== (Math|Random|RandomIntegerinRange 0 1) 0)
    (for _array_element (LocalVariables|Getlocal_Num)
      (if (== _array_element faceRandom)
        (return false)))
    (Components|StaticMesh|SetStaticMesh mesh (Utilities|Array|Get(acopy) (LocalVariables|Getlocal_Mesh) (Math|Random|RandomIntegerinRange 0 4)))
    (return true)))

(fn NPCRandomHat
  (params (mesh :type Static%20Mesh%20Component%20Object%20Reference))
  (if (== (Math|Random|RandomIntegerinRange 0 1) 0)
    (return false)
    (else
      (Components|StaticMesh|SetStaticMesh mesh (Utilities|Array|Get(acopy) (LocalVariables|Getlocal_Mesh) (Math|Random|RandomIntegerinRange 0 3)))
      (return true))))

(fn NPCRandomAC
  (params (mesh :type Static%20Mesh%20Component%20Object%20Reference))
  (if (== (Math|Random|RandomIntegerinRange 0 1) 0)
    (return false)
    (else
      (Components|StaticMesh|SetStaticMesh mesh (Utilities|Array|Get(acopy) (LocalVariables|Getlocal_Mesh) (Math|Random|RandomIntegerinRange 0 3)))
      (return true))))

(fn NPCRandomSub1
  (params (mesh :type Static%20Mesh%20Component%20Object%20Reference))
  (if (== (Math|Random|RandomIntegerinRange 0 1) 0)
    (return false)
    (else
      (Components|StaticMesh|SetStaticMesh mesh (Utilities|Array|Get(acopy) (LocalVariables|Getlocal_Mesh) (Math|Random|RandomIntegerinRange 0 7)))
      (return true))))

(fn NPCRandomSub2
  (params (mesh :type Static%20Mesh%20Component%20Object%20Reference))
  (if (== (Math|Random|RandomIntegerinRange 0 1) 0)
    (return false)
    (else
      (Components|StaticMesh|SetStaticMesh mesh (Utilities|Array|Get(acopy) (LocalVariables|Getlocal_Mesh) (Math|Random|RandomIntegerinRange 0 5)))
      (return true))))