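; Game mode blueprint that holds the score, countdown timer, score ranking and minimap capture camera.
; SortRanking writes the new score into slot 5 and swap-sorts descending, while TimeDecrease sets the time to Decrease minus the current value.
; AddMinimapUI lazily spawns BP_MinimapCamera and registers actors in its scene capture's show-only list.
; Reset restores timer and score and destroys the camera, leaving the ranking intact.
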(fn ScoreAdd
  (params (add :type Integer))
  (Variables|Default|Setscore (+ add (Variables|Default|Getscore))))

(fn TimeDecrease
  (params (decrease :type Float%20%28single-precision%29))
  (Variables|Default|SetfloatTime (- decrease (Variables|Default|GetfloatTime))))

(fn GetTimeInt
  (return (Math|Float|Truncate (Variables|Default|GetfloatTime))))

(fn SortRanking
  (params (NewScore :type Integer))
  (bind _rankingscore (Variables|Default|GetRankingScore))
  (Utilities|Array|SetArrayElem (Variables|Default|GetRankingScore) 5 NewScore)
  (LocalVariables|Setwork 5)
  (while (>= (LocalVariables|Getwork) 0)
    (LocalVariables|Setwork2 (- (LocalVariables|Getwork) 1))
    (while (>= (LocalVariables|Getwork2) 0)
      (if (> (Utilities|Array|Get(acopy) (Variables|Default|GetRankingScore) (LocalVariables|Getwork)) (Utilities|Array|Get(acopy) (Variables|Default|GetRankingScore) (LocalVariables|Getwork2)))
        (bind _output_get (LocalVariables|Settemp (Utilities|Array|Get(acopy) (Variables|Default|GetRankingScore) (LocalVariables|Getwork))))
        (Utilities|Array|SetArrayElem _rankingscore (LocalVariables|Getwork) (Utilities|Array|Get(acopy) (Variables|Default|GetRankingScore) (LocalVariables|Getwork2)))
        (Utilities|Array|SetArrayElem _rankingscore (LocalVariables|Getwork2) _output_get))
      (Math|Integer|DecrementInt (LocalVariables|Getwork2)))
    (Math|Integer|DecrementInt (LocalVariables|Getwork))))

(fn CreateMinimapCamera
  (bind _returnvalue (Game|SpawnActorfromClass "/Game/MyGame/Chiga/BP/Minimap/BP_MinimapCamera.BP_MinimapCamera_C" (Math|Transform|MakeTransform "0, 0, 0" "-90.000000,0.000000, 0" "1,1,1") "Undefined" 0 0))
  (bind _output_get (Variables|Default|SetminimapCamera _returnvalue))
  (Class|SceneCaptureComponent|ClearHiddenComponents (Variables|/Game/MyGame/Chiga/BP/Minimap/BP_MinimapCamera.BP_MinimapCamera_C|GetSceneCaptureComponent2D _output_get)))

(fn AddMinimapUI
  (params (addActor :type Actor%20Object%20Reference))
  (bind _minimapcamera (Variables|Default|GetminimapCamera))
  (if (Utilities|IsValid _minimapcamera)
    _
    (else
      (CallFunction|CreateMinimapCamera)))
  (Utilities|Array|Add (Variables|/Script/Engine.SceneCaptureComponent|GetShowOnlyActors (Variables|/Game/MyGame/Chiga/BP/Minimap/BP_MinimapCamera.BP_MinimapCamera_C|GetSceneCaptureComponent2D _minimapcamera)) addActor))

(fn Reset
  (Variables|Default|SetfloatTime 1.8e+02)
  (Variables|Default|SetintTime 180)
  (Variables|Default|Setscore 0)
  (if (Utilities|IsValid (Variables|Default|GetminimapCamera))
    (Actor|DestroyActor (Variables|Default|GetminimapCamera))))