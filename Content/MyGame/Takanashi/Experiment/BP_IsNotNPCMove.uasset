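; Behavior Tree decorator that checks whether an NPC's pawn is away from its target point, treating arrival as the NPC not moving.
; It compares the TargetLocation blackboard vector to the pawn's location, passing only when they differ beyond a small tolerance.
; The owner is cast to BP_DetourCrowdAIController once and cached for later checks.
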(fn PerformConditionCheck
  (params (OwnerActor :type Actor%20Object%20Reference))
  (if (!= (Variables|Default|GetDetourCrowdAIController) 0)
    _
    (else
      (bind _asbp_detour_crowd_aicontroller (Utilities|Casting|CastToBP_DetourCrowdAIController OwnerActor))
      (Variables|Default|SetDetourCrowdAIController _asbp_detour_crowd_aicontroller)))
  (return (not (Math|Vector|Equal(Vector) (AI|Components|Blackboard|GetValueasVector (AI|GetBlackboard (Variables|Default|GetDetourCrowdAIController)) (Variables|Default|GetTargetLocation)) (Transformation|GetActorLocation (Pawn|GetControlledPawn (Variables|Default|GetDetourCrowdAIController))) 1.0))))