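; Behavior tree task that makes a crowd NPC leave the field and spawns an NPC as it goes.
; It caches the BP_DetourCrowdAIController, gets a leave point from it and moves the pawn there, skipping the move if the controller's Destroy flag is set.
; It then calls SpawnNPC with that point, destroys the pawn and finishes; comments describe both random picks as reproducible.
; A failed move never finishes the task.
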(event EventReceiveExecute
  (params (OwnerActor :type Actor%20Object%20Reference))
  (if (!= (Variables|Default|GetDetourCrowdAIController) 0)
    _
    (else
      (bind _asbp_detour_crowd_aicontroller (Utilities|Casting|CastToBP_DetourCrowdAIController OwnerActor))
      (Variables|Default|SetDetourCrowdAIController _asbp_detour_crowd_aicontroller)))
  ;[1 1 1] 再現性のあるランダムなLeavePointを探す
  (bind _leavepoint (Default|GetLeavePoint (Variables|Default|GetDetourCrowdAIController)))
  (if (Variables|/Game/MyGame/Takanashi/BluePrint/BP_DetourCrowdAIController.BP_DetourCrowdAIController_C|GetDestroy (Variables|Default|GetDetourCrowdAIController))
    _
    (else
      ;[1 1 1] LeavePointへ向かう
      (AI|AIMoveTo (Pawn|GetControlledPawn (Variables|Default|GetDetourCrowdAIController)) "0, 0, 0" _leavepoint 1e+02 true
        (:OnSuccess
          _))))
  ;[1 1 1] 到着したら再現性のあるランダムなNPCを生成する
  (Default|SpawnNPC (Variables|Default|GetDetourCrowdAIController) _leavepoint)
  (Actor|DestroyActor (Pawn|GetControlledPawn (Variables|Default|GetDetourCrowdAIController)))
  (AI|BehaviorTree|FinishExecute true))