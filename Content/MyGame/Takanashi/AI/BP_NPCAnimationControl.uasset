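; Behavior tree service that cuts animation and shadow cost for distant NPCs.
; On activation it caches the controlled Character and player pawn 0.
; Each tick it compares their distance to MaxLength, disabling the mesh's skeleton update and shadow casting at or beyond it, and restoring both when closer.
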(event EventReceiveActivationAI
  (params (OwnerController :type AI%20Controller%20Object%20Reference) (ControlledPawn :type Pawn%20Object%20Reference))
  (bind _ascharacter (Utilities|Casting|CastToCharacter ControlledPawn))
  (Variables|Default|SetCharactor _ascharacter)
  (Variables|Default|SetPlayer (Game|Player|GetPlayerPawn 0)))

(event EventTick
  (params (OwnerActor :type Actor%20Object%20Reference) (DeltaSeconds :type Float%20%28single-precision%29))
  (bind _charactor (Variables|Default|GetCharactor))
  (bind _mesh (Variables|/Script/Engine.Character|GetMesh _charactor))
  (if (>= (Math|Vector|VectorLength (- (Transformation|GetActorLocation (Variables|Default|GetCharactor)) (Transformation|GetActorLocation (Variables|Default|GetPlayer)))) (Variables|Default|GetMaxLength))
    (Variables|/Script/Engine.SkeletalMeshComponent|SetbNoSkeletonUpdate _mesh true)
    (Rendering|SetCastShadow _mesh false)
    (else
      (Variables|/Script/Engine.SkeletalMeshComponent|SetbNoSkeletonUpdate _mesh false)
      (Rendering|SetCastShadow _mesh true))))