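; BP_SuspiciouslyWait is an AI behavior tree task that makes an agent pause briefly when flagged to wait suspiciously.
; On execute it casts the owner to BP_DetourCrowdAIController, caching the reference for reuse.
; If the controller's SuspiciouslyWait flag is set, it clears it and waits a second before finishing successfully; otherwise it succeeds immediately.
; A failed cast leaves the task unfinished.
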(event EventReceiveExecute
  (params (OwnerActor :type Actor%20Object%20Reference))
  (if (!= (Variables|Default|GetDetourCrowdAIController) 0)
    _
    (else
      (bind _asbp_detour_crowd_aicontroller (Utilities|Casting|CastToBP_DetourCrowdAIController OwnerActor))
      (Variables|Default|SetDetourCrowdAIController _asbp_detour_crowd_aicontroller)))
  (if (Variables|/Game/MyGame/Takanashi/BluePrint/BP_DetourCrowdAIController.BP_DetourCrowdAIController_C|GetSuspiciouslyWait (Variables|Default|GetDetourCrowdAIController))
    (Variables|/Game/MyGame/Takanashi/BluePrint/BP_DetourCrowdAIController.BP_DetourCrowdAIController_C|SetSuspiciouslyWait (Variables|Default|GetDetourCrowdAIController) false)
    (GameplayTasks|TaskWaitDelay 0 1.0
      (:OnFinish
        _)))
  (AI|BehaviorTree|FinishExecute true))