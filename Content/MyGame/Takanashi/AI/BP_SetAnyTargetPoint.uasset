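; Behavior Tree task for NPCs that sets the AI controller's target location from a numbered target point placed in the map.
; On tick it caches the owner as BP_DetourCrowdAIController, then searches all BP_TargetPointForNPC actors for the one matching the controller's TargetPointNum.
; It writes that actor's location to the controller's TargetLocation variable and finishes with success.
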(event EventTick
  (params (OwnerActor :type Actor%20Object%20Reference) (DeltaSeconds :type Float%20%28single-precision%29))
  (if (!= (Variables|Default|GetDetourCrowdAIController) 0)
    _
    (else
      (bind _asbp_detour_crowd_aicontroller (Utilities|Casting|CastToBP_DetourCrowdAIController OwnerActor))
      (Variables|Default|SetDetourCrowdAIController _asbp_detour_crowd_aicontroller)))
  ;[1 1 1] MapにあるTargetPointから任意のTargetPointのLocationをSetする
  (bind _outactors (Actor|GetAllActorsOfClass "/Game/MyGame/Takanashi/BluePrint/BP_TargetPointForNPC.BP_TargetPointForNPC_C"))
  (bind _array_element (Utilities|Array|ForEachLoopwithBreak _outactors :!label _label)
    (:LoopBody
      (if (== (Variables|/Game/MyGame/Takanashi/BluePrint/BP_TargetPointForNPC.BP_TargetPointForNPC_C|GetThisTargetPointNum _array_element) (Variables|/Game/MyGame/Takanashi/BluePrint/BP_DetourCrowdAIController.BP_DetourCrowdAIController_C|GetTargetPointNum (Variables|Default|GetDetourCrowdAIController)))
        (goto _label Break)))
    (:Completed
      (Variables|/Game/MyGame/Takanashi/BluePrint/BP_DetourCrowdAIController.BP_DetourCrowdAIController_C|SetTargetLocation (Variables|Default|GetDetourCrowdAIController) (Transformation|GetActorLocation _array_element))
      (AI|BehaviorTree|FinishExecute true))))