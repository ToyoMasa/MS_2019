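; Behavior tree task that picks a random destination for an NPC from the BP_TargetPointForNPC actors in the level.
; On execute it caches the owning BP_AIController, gathers the target points and writes one's location to the TargetLocation blackboard key.
; The random pick is hardcoded to the first four points found.
; The task always finishes as failed, even after writing the location.
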(event EventReceiveExecute
  (params (OwnerActor :type Actor%20Object%20Reference))
  (if (!= (Variables|Default|GetAIController) 0)
    _
    (else
      (bind _asbp_aicontroller (Utilities|Casting|CastToBP_AIController OwnerActor))
      (Variables|Default|SetAIController _asbp_aicontroller)))
  (bind _outactors (Actor|GetAllActorsOfClass "/Game/MyGame/Takanashi/BluePrint/BP_TargetPointForNPC.BP_TargetPointForNPC_C"))
  (AI|Components|Blackboard|SetValueasVector (AI|GetBlackboard (Variables|Default|GetAIController)) (Variables|Default|GetTargetLocation) (Transformation|GetActorLocation (Utilities|Array|Get(acopy) _outactors (Math|Random|RandomInteger 4))))
  (AI|BehaviorTree|FinishExecute false))