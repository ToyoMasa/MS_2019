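; BP_IsNPCMove is a Behavior Tree decorator that checks whether an NPC is away from its target location.
; It passes when the TargetLocation blackboard vector differs from the controlled pawn's location beyond a small tolerance.
; The owner is cast to BP_AIController and cached in a variable on first use, so later checks reuse it.
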(fn PerformConditionCheck
  (params (OwnerActor :type Actor%20Object%20Reference))
  (if (!= (Variables|Default|GetAIController) 0)
    _
    (else
      (bind _asbp_aicontroller (Utilities|Casting|CastToBP_AIController OwnerActor))
      (Variables|Default|SetAIController _asbp_aicontroller)))
  (return (not (Math|Vector|Equal(Vector) (AI|Components|Blackboard|GetValueasVector (AI|GetBlackboard (Variables|Default|GetAIController)) (Variables|Default|GetTargetLocation)) (Transformation|GetActorLocation (Pawn|GetControlledPawn (Variables|Default|GetAIController))) 0.1))))