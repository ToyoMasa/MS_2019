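; Behavior tree task that gives an NPC's crowd AI controller a random, reproducible destination from the map's target points.
; On execute, it casts the owner to BP_DetourCrowdAIController on first use and caches it.
; It picks one BP_TargetPointForNPC using the seeded RandomStream on the GM_MyGame game instance, writes its location to the controller's TargetLocation and finishes successfully.
; A failed cast leaves the task without a FinishExecute call.
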(event EventReceiveExecute
  (params (OwnerActor :type Actor%20Object%20Reference))
  (if (!= (Variables|Default|GetDetourCrowdAIController) 0)
    _
    (else
      (bind _asbp_detour_crowd_aicontroller (Utilities|Casting|CastToBP_DetourCrowdAIController OwnerActor))
      (Variables|Default|SetDetourCrowdAIController _asbp_detour_crowd_aicontroller)))
  ;[1 1 1] MapにあるTargetPointから再現性のあるランダムなLocationをSetする
  (bind _outactors (Actor|GetAllActorsOfClass "/Game/MyGame/Takanashi/BluePrint/BP_TargetPointForNPC.BP_TargetPointForNPC_C"))
  (bind _asgm_my_game (Utilities|Casting|CastToGM_MyGame (Game|GetGameInstance)))
  (Variables|/Game/MyGame/Takanashi/BluePrint/BP_DetourCrowdAIController.BP_DetourCrowdAIController_C|SetTargetLocation (Variables|Default|GetDetourCrowdAIController) (Transformation|GetActorLocation (Utilities|Array|Get(acopy) _outactors (Class|KismetMathLibrary|RandomIntegerfromStream (Utilities|Array|Length _outactors) (Variables|/Game/MyGame/BP/GM_MyGame.GM_MyGame_C|GetrandomStream _asgm_my_game)))))
  (AI|BehaviorTree|FinishExecute true))