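; Behavior tree tick node that updates leave and suspicious-wait flags on the crowd AI's BP_DetourCrowdAIController.
; An accumulated timer sets LeaveTheField once the controller's LeaveTime is reached.
; Until then, an active CriminalStartUp runs a short timer that sets SuspiciouslyWait, resetting while that flag is set.
; DoOnce gates each flag change, which restarts brain logic to interrupt running tasks such as BP_MoveToTargetPoint.
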(event EventTick
  (params (OwnerActor :type Actor%20Object%20Reference) (DeltaSeconds :type Float%20%28single-precision%29))
  (if (!= (Variables|Default|GetDetourCrowdAIController) 0)
    _
    (else
      (bind _asbp_detour_crowd_aicontroller (Utilities|Casting|CastToBP_DetourCrowdAIController OwnerActor))
      (Variables|Default|SetDetourCrowdAIController _asbp_detour_crowd_aicontroller)))
  ;[1 1 1] 離脱するかのフラグ
  (bind _output_get (Variables|Default|SetLeaveTime (+ (Variables|Default|GetLeaveTime) DeltaSeconds)))
  (if (>= _output_get (Variables|/Game/MyGame/Takanashi/BluePrint/BP_DetourCrowdAIController.BP_DetourCrowdAIController_C|GetLeaveTime (Variables|Default|GetDetourCrowdAIController)))
    (Utilities|FlowControl|DoOnce false
      (:Completed
        (Variables|/Game/MyGame/Takanashi/BluePrint/BP_DetourCrowdAIController.BP_DetourCrowdAIController_C|SetLeaveTheField (Variables|Default|GetDetourCrowdAIController) true)
        (Class|BrainComponent|RestartLogic (Variables|/Script/AIModule.AIController|GetBrainComponent (Variables|Default|GetDetourCrowdAIController)))))
    (elif (Variables|/Game/MyGame/Takanashi/BluePrint/BP_DetourCrowdAIController.BP_DetourCrowdAIController_C|GetCriminalStartUp (Variables|Default|GetDetourCrowdAIController))
      (if (Variables|/Game/MyGame/Takanashi/BluePrint/BP_DetourCrowdAIController.BP_DetourCrowdAIController_C|GetSuspiciouslyWait (Variables|Default|GetDetourCrowdAIController))
        (Variables|Default|SetCriminalTime 0.0)
        (goto _label Reset)
        (else
          (bind _output_get_2 (Variables|Default|SetCriminalTime (+ (Variables|Default|GetCriminalTime) DeltaSeconds)))
          (if (>= _output_get_2 1.0)
            (Utilities|FlowControl|DoOnce false :!label _label
              (:Completed
                (Variables|/Game/MyGame/Takanashi/BluePrint/BP_DetourCrowdAIController.BP_DetourCrowdAIController_C|SetSuspiciouslyWait (Variables|Default|GetDetourCrowdAIController) true)
                (Class|BrainComponent|RestartLogic (Variables|/Script/AIModule.AIController|GetBrainComponent (Variables|Default|GetDetourCrowdAIController))) ; BP_MoveToTargetPointを中断するため
              ))))))))