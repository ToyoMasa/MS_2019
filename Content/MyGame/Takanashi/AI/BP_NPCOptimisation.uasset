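; Behavior Tree service that optimises an NPC character's mesh cost by its distance to the player.
; On AI activation it caches the controlled Character and the player pawn.
; Each tick it compares their distance to fractions of MaxLength, forcing progressively coarser skeletal mesh LODs.
; Beyond half of MaxLength it also stops skeleton updates and shadow casting, restoring both when closer.
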(event EventReceiveActivationAI
  (params (OwnerController :type AI%20Controller%20Object%20Reference) (ControlledPawn :type Pawn%20Object%20Reference))
  (bind _ascharacter (Utilities|Casting|CastToCharacter ControlledPawn))
  (Variables|Default|SetCharactor _ascharacter)
  (Variables|Default|SetPlayer (Game|Player|GetPlayerPawn 0)))

(event EventTick
  (params (OwnerActor :type Actor%20Object%20Reference) (DeltaSeconds :type Float%20%28single-precision%29))
  (bind _charactor (Variables|Default|GetCharactor))
  (bind _player (Variables|Default|GetPlayer))
  (bind _maxlength (Variables|Default|GetMaxLength))
  (bind _charactor_2 (Variables|Default|GetCharactor))
  (bind _returnvalue (Transformation|GetActorLocation _player))
  (bind _returnvalue_2 (Transformation|GetActorLocation _charactor))
  (bind _mesh (Variables|/Script/Engine.Character|GetMesh _charactor_2))
  (bind _returnvalue_3 (- _returnvalue_2 _returnvalue))
  (bind _returnvalue_4 (Math|Vector|VectorLength _returnvalue_3))
  ;[1 1 1] 段階的にポリゴン数を削り、アニメーションとシャドウの停止をする
  (if (<= _returnvalue_4 (* _maxlength 0.1))
    (Components|SkinnedMesh|SetForcedLOD _mesh 1)
    (Variables|/Script/Engine.SkeletalMeshComponent|SetbNoSkeletonUpdate _mesh false :!label _label)
    (Rendering|SetCastShadow _mesh true)
    (elif (<= _returnvalue_4 (* _maxlength 0.2))
      (Components|SkinnedMesh|SetForcedLOD _mesh 2)
      (goto _label)
      (elif (<= _returnvalue_4 (* _maxlength 0.3))
        (Components|SkinnedMesh|SetForcedLOD _mesh 3)
        (goto _label)
        (elif (<= _returnvalue_4 (* _maxlength 0.4))
          (Components|SkinnedMesh|SetForcedLOD _mesh 4)
          (goto _label)
          (elif (<= _returnvalue_4 (* _maxlength 0.5))
            (Components|SkinnedMesh|SetForcedLOD _mesh 5)
            (goto _label)
            (else
              (Components|SkinnedMesh|SetForcedLOD _mesh 5)
              (Variables|/Script/Engine.SkeletalMeshComponent|SetbNoSkeletonUpdate _mesh true)
              (Rendering|SetCastShadow _mesh false))))))))