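; Behavior tree node that makes a detour-crowd AI react when its criminal start-up state begins.
; Each tick it reads CriminalStartUp from the owning BP_DetourCrowdAIController, which it casts and caches on first use.
; When the flag turns true, it restarts the brain component's logic to interrupt BP_MoveToTargetPoint.
; A DoOnce limits this to one restart and re-arms when the flag is false.
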(event EventTick
  (params (OwnerActor :type Actor%20Object%20Reference) (DeltaSeconds :type Float%20%28single-precision%29))
  (if (!= (Variables|Default|GetDetourCrowdAIController) 0)
    _
    (else
      (bind _asbp_detour_crowd_aicontroller (Utilities|Casting|CastToBP_DetourCrowdAIController OwnerActor))
      (Variables|Default|SetDetourCrowdAIController _asbp_detour_crowd_aicontroller)))
  (if (Variables|/Game/MyGame/Takanashi/BluePrint/BP_DetourCrowdAIController.BP_DetourCrowdAIController_C|GetCriminalStartUp (Variables|Default|GetDetourCrowdAIController))
    (Utilities|FlowControl|DoOnce false :!label _label
      (:Completed
        (Class|BrainComponent|RestartLogic (Variables|/Script/AIModule.AIController|GetBrainComponent (Variables|Default|GetDetourCrowdAIController))) ; BP_MoveToTargetPointを中断するため
      ))
    (else
      (goto _label Reset))))