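; Behavior tree task that sends a crowd AI character to the nearest normal NPC for pickpocketing.
; On execute it caches the DetourCrowd AI controller, scans all NormalNPC actors by distance and doubles the pawn's walk speed for the approach.
; Reaching the target clears the controller's Pickpocket flag, sets LeaveTheField, finishes successfully and restarts brain logic.
; A failed move has no handler, so the task does not finish in that case.
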(event EventReceiveExecute
  (params (OwnerActor :type Actor%20Object%20Reference))
  (if (!= (Variables|Default|GetDetourCrowdAIController) 0)
    _
    (else
      (bind _asbp_detour_crowd_aicontroller (Utilities|Casting|CastToBP_DetourCrowdAIController OwnerActor))
      (Variables|Default|SetDetourCrowdAIController _asbp_detour_crowd_aicontroller)))
  ;[1 1 1] 一番近いNormalNPCを探す
  (bind _outactors (Actor|GetAllActorsOfClass "/Game/MyGame/Toyomura/Blueprints/NPC/BP_NormalNPC.BP_NormalNPC_C"))
  (for (_array_element _array_index) _outactors
    (if (<= (Transformation|GetDistanceTo OwnerActor _array_element) (Variables|Default|GetDistance))
      (Variables|Default|SetDistance (Transformation|GetDistanceTo OwnerActor _array_element))
      (Variables|Default|SetNormalNPCIndex _array_index)))
  ;[1 1 1] 歩行速度を上昇させNormalNPCに接近し、接触したらLeavePointへ向かう
  (bind _ascharacter (Utilities|Casting|CastToCharacter (Pawn|GetControlledPawn (Variables|Default|GetDetourCrowdAIController))))
  (Variables|/Script/Engine.CharacterMovementComponent|SetMaxWalkSpeed (Variables|/Script/Engine.Character|GetCharacterMovement _ascharacter) (* (Variables|/Script/Engine.CharacterMovementComponent|GetMaxWalkSpeed (Variables|/Script/Engine.Character|GetCharacterMovement _ascharacter)) 2.0))
  (AI|AIMoveTo (Pawn|GetControlledPawn (Variables|Default|GetDetourCrowdAIController)) "0, 0, 0" (Utilities|Array|Get(acopy) _outactors (Variables|Default|GetNormalNPCIndex)) 5e+01 true
    (:OnSuccess
      (Variables|/Game/MyGame/Takanashi/BluePrint/BP_DetourCrowdAIController.BP_DetourCrowdAIController_C|SetPickpocket (Variables|Default|GetDetourCrowdAIController) false)
      (Variables|/Game/MyGame/Takanashi/BluePrint/BP_DetourCrowdAIController.BP_DetourCrowdAIController_C|SetLeaveTheField (Variables|Default|GetDetourCrowdAIController) true)
      (AI|BehaviorTree|FinishExecute true)
      (Class|BrainComponent|RestartLogic (Variables|/Script/AIModule.AIController|GetBrainComponent (Variables|Default|GetDetourCrowdAIController))))))