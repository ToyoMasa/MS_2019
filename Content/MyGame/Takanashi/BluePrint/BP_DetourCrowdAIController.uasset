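; Detour crowd AI controller that runs a behavior tree for NPCs, with state for a criminal start-up move to a numbered target point.
; On BeginPlay it starts the blackboard and tree, then draws a random LeaveTime from the GM_MyGame game instance's seeded stream.
; NPCMoveTo and ResetState set or clear the criminal flag and target point, restarting the brain logic each time.
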(event EventBeginPlay
  (Class|AIController|UseBlackboard "/Game/MyGame/Takanashi/AI/Blackboard.Blackboard")
  (AI|RunBehaviorTree "/Game/MyGame/Takanashi/AI/BehaviorTree.BehaviorTree")
  (bind _asgm_my_game (Utilities|Casting|CastToGM_MyGame (Game|GetGameInstance)))
  (Variables|Default|SetLeaveTime (Math|Random|RandomFloatinRangefromStream 3.0 4.0 (Variables|/Game/MyGame/BP/GM_MyGame.GM_MyGame_C|GetrandomStream _asgm_my_game))))

(event EventTick
  (params (DeltaSeconds :type Float%20%28single-precision%29)))

(fn ConstructionScript)

(fn NPCMoveto
  (params (TargetPointNum :type Integer))
  (Variables|Default|SetCriminalStartUp true)
  (Variables|Default|SetTargetPointNum TargetPointNum)
  (Class|BrainComponent|RestartLogic (Variables|Default|GetBrainComponent)))

(fn ResetState
  (Variables|Default|SetCriminalStartUp false)
  (Variables|Default|SetTargetPointNum -1)
  (Class|BrainComponent|RestartLogic (Variables|Default|GetBrainComponent)))