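; BP_PrisonStageCamera is a stage camera that travels along a series of NPC locations.
; On BeginPlay it becomes the player's view target and triggers the first BP_TestNPCSpawn to spawn NPCs.
; Once IsStart is set, Tick lerps it between successive locations, flagging the current NPC's SpotChange from each segment's midpoint, except on the last location.
; IsEnd halts it when no NPCs exist or the count is reached.
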(event EventBeginPlay
  (Game|Player|SetViewTargetwithBlend (Game|GetPlayerController 0) self 0.0 "VTBlend_Linear" 0.0 false)
  (Variables|Default|SetStartPos (Transformation|GetActorLocation))
  (bind _outactors (Actor|GetAllActorsOfClass "/Game/MyGame/Toyomura/Blueprints/NPC/BP_TestNPCSpawn.BP_TestNPCSpawn_C"))
  (Default|Spawn (Utilities|Array|Get(acopy) _outactors))
  (bind _output_get (Variables|Default|SetSpawnNPC (Utilities|Array|Get(acopy) _outactors)))
  (Variables|Default|SetEndpos (Utilities|Array|Get(acopy) (Variables|/Game/MyGame/Toyomura/Blueprints/NPC/BP_TestNPCSpawn.BP_TestNPCSpawn_C|GetNPCLocations _output_get)))
  (if (== (Utilities|Array|Length (Variables|/Game/MyGame/Toyomura/Blueprints/NPC/BP_TestNPCSpawn.BP_TestNPCSpawn_C|GetNPCs _output_get)) 0)
    (Variables|Default|SetisEnd true)))

(event Collision|EventActorBeginOverlap
  (params (OtherActor :type Actor%20Object%20Reference)))

(event EventTick
  (params (DeltaSeconds :type Float%20%28single-precision%29))
  (bind _spawnnpc (Variables|Default|GetSpawnNPC))
  (bind _npccnt (Variables|Default|GetnpcCnt))
  (bind _output_get (Variables|Default|SetdeltaTime DeltaSeconds))
  (if (not (Variables|Default|GetisEnd))
    (if (Variables|Default|GetisStart)
      (bind _output_get_2 (Variables|Default|SetTime (Math|Float|Clamp(Float) (+ (* _output_get (Variables|Default|GettimeAdd)) (Variables|Default|GetTime)))))
      (if (>= _output_get_2 0.5)
        (if (< _npccnt (- (Utilities|Array|Length (Variables|/Game/MyGame/Toyomura/Blueprints/NPC/BP_TestNPCSpawn.BP_TestNPCSpawn_C|GetNPCLocations _spawnnpc)) 1))
          (Variables|/Game/MyGame/Toyomura/Blueprints/NPC/BP_NPCResultHand.BP_NPCResultHand_C|SetSpotChange (Utilities|Array|Get(acopy) (Variables|/Game/MyGame/Toyomura/Blueprints/NPC/BP_TestNPCSpawn.BP_TestNPCSpawn_C|GetNPCs _spawnnpc) _npccnt) true)))
      (Transformation|SetActorLocation (Math|Vector|Lerp(Vector) (Variables|Default|GetStartPos) (Variables|Default|GetEndpos) _output_get_2) false false)
      (if (>= _output_get_2 1.0)
        (Variables|Default|SetTime 0.0)
        (if (!= (Variables|Default|GetnpcCnt) (Utilities|Array|Length (Variables|/Game/MyGame/Toyomura/Blueprints/NPC/BP_TestNPCSpawn.BP_TestNPCSpawn_C|GetNPCs (Variables|Default|GetSpawnNPC))))
          (bind _result (Math|Integer|IncrementInt (Variables|Default|GetnpcCnt))
            (:%20%20
              (Variables|Default|SetStartPos (Variables|Default|GetEndpos))
              (Variables|Default|SetEndpos (Utilities|Array|Get(acopy) (Variables|/Game/MyGame/Toyomura/Blueprints/NPC/BP_TestNPCSpawn.BP_TestNPCSpawn_C|GetNPCLocations (Variables|Default|GetSpawnNPC)) _result))))
          (else
            (Variables|Default|SetisEnd true)))))))

(fn ConstructionScript)