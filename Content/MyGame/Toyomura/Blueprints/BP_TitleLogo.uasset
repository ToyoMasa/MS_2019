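; BP_TitleLogo is the title logo actor, showing front and back faces through two widget components that hold W_Title and W_Title2.
; Tick spins the back component, Widget1, around yaw at a constant frame-rate-independent speed.
; The Fade function plays the FadeOut animation on both user widgets.
; The Fadeout event is an empty stub and does not call Fade.
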(event Custom|Fadeout)

(event EventBeginPlay)

(event Collision|EventActorBeginOverlap
  (params (OtherActor :type Actor%20Object%20Reference)))

(event EventTick
  (params (DeltaSeconds :type Float%20%28single-precision%29))
  (bind _widget1 (Variables|Default|GetWidget1))
  (bind _returnvalue (Transformation|GetWorldRotation _widget1))
  (Transformation|SetWorldRotation _widget1 (Math|Rotator|MakeRotator (.roll _returnvalue) (.pitch _returnvalue) (+ (* DeltaSeconds 2e+01) (.yaw _returnvalue))) false false))

(fn ConstructionScript)

(fn Fade
  (Utilities|FlowControl|Sequence
    (:then_0
      ;[1 1 1] 表面のフェード処理
      (bind _asw_title (Utilities|Casting|CastToW_Title (UserInterface|GetUserWidgetObject (Variables|Default|GetWidget))))
      (UserInterface|Animation|PlayAnimation _asw_title (Variables|/Game/MyGame/Toyomura/Blueprints/Widgets/W_Title.W_Title_C|GetFadeOut _asw_title) 0.0 1 "Forward" 1.0))
    (:then_1
      ;[1 1 1] 裏面のフェード処理
      (bind _asw_title_2 (Utilities|Casting|CastToW_Title2 (UserInterface|GetUserWidgetObject (Variables|Default|GetWidget1))))
      (UserInterface|Animation|PlayAnimation _asw_title_2 (Variables|/Game/MyGame/Toyomura/Blueprints/Widgets/W_Title2.W_Title2_C|GetFadeOut _asw_title_2) 0.0 1 "Forward" 1.0))))