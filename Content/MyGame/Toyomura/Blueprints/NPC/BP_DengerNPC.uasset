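; BP_DengerNPC is a child NPC Blueprint that can change type when a search on it ends.
; It sets its starting type on BeginPlay, and SearchEnd may switch it before calling the parent logic, depending on the drone's level.
; The switch never happens at level 0, grows likelier through levels 1 and 2, and is certain at 3 and 4.
; A switch, or a SearchDirect event, marks the NPC as directly searched.
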(event EventBeginPlay
  (|CallParentFunction)
  (CallFunction|ChangeType "NewEnumerator1"))

(event Collision|EventActorBeginOverlap
  (params (OtherActor :type Actor%20Object%20Reference)))

(event EventTick
  (params (DeltaSeconds :type Float%20%28single-precision%29))
  (|CallParentFunction DeltaSeconds))

(event EventSearchEnd
  (bind _getdrone (Variables|Default|GetGetDrone))
  (bind _level (Variables|/Game/MyGame/Toyomura/Blueprints/Player/BP_PlayerDrone.BP_PlayerDrone_C|GetLevel _getdrone))
  (switch int _level
    (:Default
      (|CallParentFunction :!label _label))
    (:0
      (goto _label))
    (:1
      (if (== (Math|Random|RandomInteger (- 4 _level)) 0) :!label _label_2
        (Variables|Default|Settype "NewEnumerator0")
        (|CallParentFunction)
        (Variables|Default|SetisDirectSearched true)
        (else
          (|CallParentFunction))))
    (:2
      (goto _label_2))
    (:3
      (goto _label_2))
    (:4
      (Variables|Default|Settype "NewEnumerator0")
      (|CallParentFunction)
      (Variables|Default|SetisDirectSearched true))))

(event EventSearchDirect
  (Variables|Default|SetisDirectSearched true))

(fn ConstructionScript
  (|CallParentFunction))