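; BP_TestNPCSpawn is a test actor that spawns an NPC result hand from stored NPC data.
; On BeginPlay it casts the game instance to GM_MyGame and, if NPCDatas has entries, prints their count.
; It then spawns BP_NPCResultHand at its own location and passes the first entry to MaterialLoad.
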(event EventBeginPlay
  (bind _asgm_my_game (Utilities|Casting|CastToGM_MyGame (Game|GetGameInstance)))
  (if (> (Utilities|Array|Length (Variables|/Game/MyGame/BP/GM_MyGame.GM_MyGame_C|GetNPCDatas _asgm_my_game)) 0)
    (Development|PrintString (Utilities|String|ToString(Integer) (Utilities|Array|Length (Variables|/Game/MyGame/BP/GM_MyGame.GM_MyGame_C|GetNPCDatas _asgm_my_game))))
    (bind _returnvalue (Game|SpawnActorfromClass "/Game/MyGame/Toyomura/Blueprints/NPC/BP_NPCResultHand.BP_NPCResultHand_C" (Math|Transform|MakeTransform (Transformation|GetActorLocation) "0, 0, 0" "1,1,1") "Undefined" 0 0))
    (Default|MaterialLoad _returnvalue (Utilities|Array|Get(acopy) (Variables|/Game/MyGame/BP/GM_MyGame.GM_MyGame_C|GetNPCDatas _asgm_my_game)))))

(event Collision|EventActorBeginOverlap
  (params (OtherActor :type Actor%20Object%20Reference)))

(event EventTick
  (params (DeltaSeconds :type Float%20%28single-precision%29)))

(fn ConstructionScript)