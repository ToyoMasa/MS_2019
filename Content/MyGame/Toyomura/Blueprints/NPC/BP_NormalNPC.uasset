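; BP_NormalNPC is a child NPC Blueprint that sets its type to the first enumerator on BeginPlay and extends the inherited search events.
; When SearchDirect fires and the NPC is not yet searched, it calls Search with a fixed value.
; Search runs the parent logic and then flags the NPC as directly searched.
; Tick, SearchEnd and the construction script only pass through to the parent.
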(event EventBeginPlay
  (|CallParentFunction)
  (CallFunction|ChangeType "NewEnumerator0"))

(event Collision|EventActorBeginOverlap
  (params (OtherActor :type Actor%20Object%20Reference)))

(event EventTick
  (params (DeltaSeconds :type Float%20%28single-precision%29))
  (|CallParentFunction DeltaSeconds))

(event EventSearch
  (params (Search :type Float%20%28single-precision%29))
  (|CallParentFunction Search)
  (Variables|Default|SetisDirectSearched true))

(event EventSearchEnd
  (|CallParentFunction))

(event EventSearchDirect
  (|CallParentFunction)
  (if (not (Variables|Default|GetisSearched))
    (CallFunction|Search 1e+02)))

(fn ConstructionScript
  (|CallParentFunction))