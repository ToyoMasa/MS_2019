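; BP_CriminalNPC is the criminal NPC, which sets its type on BeginPlay and spawns warning holograms while out of view.
; Every Tick, CreateHologram spawns a BP_Warning_Child at the mesh transform if the NPC was not recently rendered, then waits a random cooldown counted by fixed per-frame increments.
; SearchDirect passes a judgement, marks the NPC searched and expires it shortly after; destruction removes its UI.
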(event EventBeginPlay
  (|CallParentFunction)
  (CallFunction|ChangeType "NewEnumerator2"))

(event Collision|EventActorBeginOverlap
  (params (OtherActor :type Actor%20Object%20Reference))
  (|CallParentFunction OtherActor) ; This node is disabled and will not be called.\nDrag off pins to build functionality.
)

(event EventTick
  (params (DeltaSeconds :type Float%20%28single-precision%29))
  (|CallParentFunction DeltaSeconds)
  (CallFunction|CreateHologram))

(event EventSearchDirect
  (CallFunction|SearchJudgement "NewEnumerator2")
  (Utilities|FlowControl|Sequence
    (:then_0
      (Variables|Default|SetisSearched true))
    (:then_1
      (Actor|SetLifeSpan 2.0))))

(event EventDestroyed
  (CallFunction|DestroyUI))

(fn ConstructionScript
  (|CallParentFunction))

(fn CreateHologram
  (if (Variables|Default|GetisHoloGram)
    (bind _output_get (Variables|Default|SettimeCnt (+ (Variables|Default|GettimeCnt) 0.016667)))
    (if (>= _output_get (Variables|Default|GettimeMax))
      (Variables|Default|SettimeCnt 0.0)
      (Variables|Default|SetisHoloGram false))
    (elif (not (Class|Actor|WasRecentlyRendered 0.2))
      ;[1 1 1] Hologramを作成
      (bind _returnvalue (Game|SpawnActorfromClass "/Game/MyGame/Chiga/BP/Hologram/BP_Warning_Child.BP_Warning_Child_C" (Transformation|GetWorldTransform (Variables|Character|GetMesh)) "Undefined" 0 0))
      (Default|Init _returnvalue self)
      (Variables|Default|SetisHoloGram true)
      (Variables|Default|SettimeMax (Math|Random|RandomFloatinRange 1e+01 25.0)))))