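; Base NPC that the player's drone scans to reveal whether it is normal, dangerous or criminal.
; While rendered within range of the drone, Tick builds scan progress; completion triggers type-colored effects, score and drone EXP.
; It spawns a minimap marker and gauge, randomizes its appearance, and drives a drone-only overlay mesh with custom depth.
; AIWait stops the AI's movement, turns it toward the player, then judges it Normal and restarts its logic.
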(event OnComponentBeginOverlap(Sphere)
  (params (OverlappedComponent :type Primitive%20Component%20Object%20Reference) (OtherActor :type Actor%20Object%20Reference) (OtherComp :type Primitive%20Component%20Object%20Reference) (OtherBodyIndex :type Integer) (bFromSweep :type Boolean) (SweepResult :type Hit%20Result%20Structure%20%28by%20ref%29))
  (Utilities|Casting|CastToBP_PlayerHuman OtherActor)
  (Variables|Default|SetisHit true))

(event OnComponentEndOverlap(Sphere)
  (params (OverlappedComponent :type Primitive%20Component%20Object%20Reference) (OtherActor :type Actor%20Object%20Reference) (OtherComp :type Primitive%20Component%20Object%20Reference) (OtherBodyIndex :type Integer))
  (Utilities|Casting|CastToBP_PlayerHuman OtherActor)
  (Variables|Default|SetisHit false))

(event Custom|AIWait
  (params (NPC :type Actor%20Object%20Reference))
  (bind _returnvalue (AI|GetAIController NPC))
  (bind _gage (Variables|Default|GetGage))
  (bind _gage_2 (Variables|Default|GetGage))
  ;[1 1 1] ビヘイビアツリーを一定時間停止する
  (Variables|Default|SetCheckOn true)
  (AI|Navigation|StopMovement _returnvalue)
  (Utilities|FlowControl|Delay 2.5)
  (Variables|/Game/MyGame/Chiga/BP/Particle/BP_GageParticle.BP_GageParticle_C|SetisWhat _gage_2 true)
  (Variables|/Game/MyGame/Chiga/BP/Particle/BP_GageParticle.BP_GageParticle_C|SetWhatType _gage_2 true)
  (Variables|Default|SetCheckOn false)
  (Variables|Default|SetIsByeBye true)
  (Utilities|FlowControl|Delay 1.0)
  (Variables|Default|SetIsByeBye false)
  (Variables|Default|SetisDirectSearched false)
  (Utilities|FlowControl|Delay 1.0)
  (Rendering|Material|SetTextureParameterValue (Variables|/Game/MyGame/Chiga/BP/Particle/BP_GageParticle.BP_GageParticle_C|Getmaterial _gage) "Icon" (Utilities|Select :Index (Variables|Default|Gettype) :NewEnumerator0 "/Game/MyGame/Chiga/Texture/Icon/blue.blue" :NewEnumerator1 "/Game/MyGame/Chiga/Texture/Icon/blue.blue" :NewEnumerator2 "/Game/MyGame/Chiga/Texture/Icon/red.red"))
  (Variables|/Game/MyGame/Chiga/BP/Particle/BP_GageParticle.BP_GageParticle_C|SetisReturnChange _gage true)
  (Variables|/Game/MyGame/Chiga/BP/Particle/BP_GageParticle.BP_GageParticle_C|SetisChange _gage true)
  (Variables|/Game/MyGame/Chiga/BP/Particle/BP_GageParticle.BP_GageParticle_C|SetisWhat _gage false)
  (CallFunction|SearchJudgement "NewEnumerator0")
  (Class|BrainComponent|RestartLogic (Variables|/Script/AIModule.AIController|GetBrainComponent _returnvalue)))

(event EventBeginPlay
  (bind _returnvalue (Game|SpawnActorfromClass "/Game/MyGame/Chiga/BP/Minimap/BP_MinimapUI.BP_MinimapUI_C" (Math|Transform|MakeTransform "0, 0, 0" "0, 0, 0" "1,1,1") "Undefined" 0 0))
  (bind _output_get (Variables|Default|SetminimapUI _returnvalue))
  (bind _asgm_my_game (Utilities|Casting|CastToGM_MyGame (Game|GetGameInstance)))
  (Default|AddMinimapUI _asgm_my_game _output_get)
  (Rendering|SetRenderCustomDepth (Variables|Character|GetMesh) true)
  (CallFunction|SkeletalInit)
  (CallFunction|GageInit)
  (CallFunction|MaterialInit))

(event EventDestroyed)

(event EventTick
  (params (DeltaSeconds :type Float%20%28single-precision%29))
  (bind _returnvalue (Game|Player|GetPlayerPawn 0))
  (bind _returnvalue_2 (Game|Player|GetPlayerPawn 0))
  (Utilities|FlowControl|Sequence
    (:then_0
      (CallFunction|GageUpdate)
      (CallFunction|MaterialUpdate)
      (CallFunction|SkeletalUpdate)
      (CallFunction|PositionUpdate (Variables|Default|GetminimapUI) self))
    (:then_1
      ;[1 1 1] 分析したかどうか
      (if (not (Variables|Default|GetisSearched))
        ;[1 1 1] プレイヤーがドローン使用中かどうか
        (bind _asbp_player_drone (Utilities|Casting|CastToBP_PlayerDrone _returnvalue))
        ;[1 1 1] 分析率取得用
        (Variables|Default|SetGetDrone _asbp_player_drone)
        ;[1 1 1] まだ分析されてないか
        (if (not (Variables|Default|GetisSearched))
          ;[1 1 1] プレイヤーとの距離チェック
          (if (> 3e+03 (Math|Vector|VectorLength (- (Transformation|GetActorLocation _returnvalue) (Transformation|GetActorLocation))))
            ;[1 1 1] カメラに写っているか
            (if (Class|Actor|WasRecentlyRendered 0.2)
              ;[1 1 1] 全て通ったら分析率を上げる
              (CallFunction|Search (* (Utilities|Array|Get(acopy) (Variables|/Game/MyGame/Toyomura/Blueprints/Player/BP_PlayerDrone.BP_PlayerDrone_C|GetSearchRate (Variables|Default|GetGetDrone)) (Variables|/Game/MyGame/Toyomura/Blueprints/Player/BP_PlayerDrone.BP_PlayerDrone_C|GetLevel (Variables|Default|GetGetDrone))) (Utilities|Time|GetWorldDeltaSeconds))))))))
    (:then_2
      ;[1 1 1] プレイヤーがドローン使用中かどうか
      (Utilities|Casting|CastToBP_PlayerDrone _returnvalue_2)
      ;[1 1 1] プレイヤーとの距離チェック
      (if (> 3e+03 (Math|Vector|VectorLength (- (Transformation|GetActorLocation _returnvalue_2) (Transformation|GetActorLocation))))
        (if (Class|Actor|WasRecentlyRendered 0.2)
          (Variables|/Game/MyGame/Chiga/BP/Particle/BP_GageParticle.BP_GageParticle_C|SetisSearch (Variables|Default|GetGage) true))))
    (:then_3
      ;[1 1 1] プレイヤーの方を向く
      (if (Variables|Default|GetCheckOn)
        (Transformation|SetActorRotation (Math|Interpolation|RInterpTo (Transformation|GetActorRotation) (Math|Rotator|MakeRotator 0.0 0.0 (.Yaw (Math|Rotator|BreakRotator (Math|Rotator|FindLookatRotation (Transformation|GetActorLocation) (Transformation|GetActorLocation (Game|Player|GetPlayerPawn 0)))))) (Utilities|Time|GetWorldDeltaSeconds) 5.0))))))

(fn ConstructionScript)

(fn SearchEnd
  (bind _gage (Variables|Default|GetGage))
  (if (not (Variables|Default|GetisSearchEnd))
    (CallFunction|Jugement)
    (Variables|Default|SetisSearchEnd true)
    (Rendering|Material|SetTextureParameterValue (Variables|/Game/MyGame/Chiga/BP/Particle/BP_GageParticle.BP_GageParticle_C|Getmaterial _gage) "Icon" (Utilities|Select :Index (Variables|Default|Gettype) :NewEnumerator0 "/Game/MyGame/Chiga/Texture/Icon/blue.blue" :NewEnumerator1 "/Game/MyGame/Chiga/Texture/Icon/red.red" :NewEnumerator2 "/Game/MyGame/Chiga/Texture/Icon/red.red"))
    (Variables|/Game/MyGame/Chiga/BP/Particle/BP_GageParticle.BP_GageParticle_C|SetisChange _gage true)
    ;[1 1 1] ACIDの経験値取得
    (Default|GetSearchEXP (Variables|Default|GetGetDrone))))

(fn Search
  (params (Search :type Float%20%28single-precision%29))
  (bind _asbp_player_drone (Utilities|Casting|CastToBP_PlayerDrone (Game|Player|GetPlayerPawn 0)))
  (if (not (Variables|/Game/MyGame/Toyomura/Blueprints/Player/BP_PlayerDrone.BP_PlayerDrone_C|GetIsHacking _asbp_player_drone))
    (Variables|/Game/MyGame/Chiga/BP/Particle/BP_GageParticle.BP_GageParticle_C|SetisSearch (Variables|Default|GetGage) true)
    (CallFunction|CreateParticle)
    (if (not (Variables|Default|GetisSearched))
      (bind _output_get (Variables|Default|SetSearchRate (+ Search (Variables|Default|GetSearchRate))))
      (if (>= _output_get 1e+02)
        (CallFunction|SearchEnd)
        (bind _asgm_my_game (Utilities|Casting|CastToGM_MyGame (Game|GetGameInstance)))
        (Default|ScoreAdd _asgm_my_game (Variables|Default|GetSearchScore))
        (Variables|Default|SetisSearched true)
        (Variables|Default|SetSearchRate (Math|Float|Clamp(Float) (Variables|Default|GetSearchRate) 0.0 1e+02))))))

(fn SearchDirect)

(fn CreateParticle
  (if (not (Variables|Default|GetisCreateParticle))
    (bind _returnvalue (Game|SpawnActorfromClass "/Game/MyGame/Chiga/BP/Particle/BP_ParticleBase.BP_ParticleBase_C" (Math|Transform|MakeTransform "0, 0, 0" "0, 0, 0" "1,1,1") "Undefined" 0 0))
    (bind _output_get (Variables|Default|SetscanParticle _returnvalue))
    (Variables|/Game/MyGame/Chiga/BP/Particle/BP_ParticleBase.BP_ParticleBase_C|SetattachActor _output_get self)
    (Variables|Default|SetisCreateParticle true)))

(fn Jugement
  (bind _scanparticle (Variables|Default|GetscanParticle))
  (bind _gage (Variables|Default|GetGage))
  (bind _material (Variables|/Game/MyGame/Chiga/BP/Particle/BP_GageParticle.BP_GageParticle_C|Getmaterial _gage))
  (if (not (Variables|Default|GetisJugment))
    (switch Utilities|FlowControl|Switch|SwitchonE_NPCType (Variables|Default|Gettype)
      (:NewEnumerator0
        (LocalVariables|Setspawn "/Game/MyGame/Chiga/BP/Particle/BP_ParticleSafe.BP_ParticleSafe_C")
        (bind _output_get (LocalVariables|SetColor "(R=0.000000,G=0.736171,B=5.000000,A=1.000000)"))
        (LocalVariables|SetScanColor _output_get))
      (:NewEnumerator1
        (LocalVariables|Setspawn "/Game/MyGame/Chiga/BP/Particle/BP_ParticleDenger.BP_ParticleDenger_C" :!label _label)
        (LocalVariables|SetColor "(R=5.000000,G=0.000000,B=1.700821,A=1.000000)")
        (LocalVariables|SetScanColor "(R=5.000000,G=0.000000,B=0.000000,A=1.000000)"))
      (:NewEnumerator2
        (goto _label)))
    (bind _returnvalue (Game|SpawnActorfromClass (LocalVariables|Getspawn) (Math|Transform|MakeTransform "0, 0, 0" "0, 0, 0" "1,1,1") "Undefined" 0 0))
    (bind _asbp_base_particle (Utilities|Casting|CastToBP_BaseParticle _returnvalue))
    (Default|SetActor _asbp_base_particle self)
    (Actor|SetLifeSpan _asbp_base_particle 3.0)
    (Rendering|Material|SetVectorParameterValue _material "ColorEm" (LocalVariables|GetColor) :!class /Script/Engine.MaterialInstanceDynamic)
    (Rendering|Material|SetVectorParameterValue _material "Color" (LocalVariables|GetScanColor) :!class /Script/Engine.MaterialInstanceDynamic)
    (if (Utilities|IsValid _scanparticle)
      _
      (else
        (CallFunction|CreateParticle)))
    (for _array_element (Variables|/Game/MyGame/Chiga/BP/Particle/BP_ParticleBase.BP_ParticleBase_C|Getmaterial _scanparticle)
      (Rendering|Material|SetVectorParameterValue _array_element "Color" (LocalVariables|GetScanColor) :!class /Script/Engine.MaterialInstanceDynamic))
    (for _array_element_2 (Variables|Default|Getmaterial)
      (Rendering|Material|SetVectorParameterValue _array_element_2 "NPCColor" (LocalVariables|GetColor) :!class /Script/Engine.MaterialInstanceDynamic))))

(fn ChangeType
  (params (type :type E_NPCType%20Enum :default "NewEnumerator0"))
  (Variables|Default|Settype type))

(fn SkeletalInit
  (bind _mesh (Variables|Character|GetMesh))
  (Class|SkinnedMeshComponent|SetSkeletalMesh (Variables|Default|GetSkeletalMesh) (Variables|/Script/Engine.SkinnedMeshComponent|GetSkeletalMesh _mesh) true)
  (Components|SkeletalMesh|SetAnimInstanceClass (Variables|Default|GetSkeletalMesh) (Variables|/Script/Engine.SkeletalMeshComponent|GetAnimClass _mesh))
  (Rendering|SetRenderCustomDepth (Variables|Character|GetMesh) true)
  (Rendering|SetCustomDepthStencilValue (Variables|Default|GetSkeletalMesh) 1)
  (for _index (range 0 (Rendering|Material|GetNumMaterials (Variables|Character|GetMesh)))
    (bind _returnvalue (Rendering|Material|CreateDynamicMaterialInstance (Variables|Default|GetSkeletalMesh) _index "/Game/MyGame/Chiga/Material/NPC/M_NPC_Inst.M_NPC_Inst" "None" :!class /Script/Engine.PrimitiveComponent))
    (Rendering|Material|SetScalarParameterValue _returnvalue "Alpha" 0.0 :!class /Script/Engine.MaterialInstanceDynamic)
    (Utilities|Array|Add (Variables|Default|Getmaterial) _returnvalue)))

(fn MaterialUpdate
  (bind _alphalength (Variables|Default|GetalphaLength))
  (for _array_element (Variables|Default|Getmaterial)
    (Rendering|Material|SetScalarParameterValue _array_element "Alpha" (/ (Variables|Default|GetSearchRate) 1e+02) :!class /Script/Engine.MaterialInstanceDynamic))
  (for _array_element_2 (Variables|Default|Getmaterials)
    (Rendering|Material|SetScalarParameterValue _array_element_2 "AlphaLength" _alphalength :!class /Script/Engine.MaterialInstanceDynamic))
  (Rendering|Material|SetScalarParameterValue (Variables|Default|GethairMaterial) "AlphaLength" _alphalength :!class /Script/Engine.MaterialInstanceDynamic)
  (Utilities|FlowControl|Sequence
    (:then_0
      (if (Variables|Default|GetisGlass)
        (Rendering|Material|SetScalarParameterValue (Variables|Default|GetGlassMaterial) "AlphaLength" _alphalength :!class /Script/Engine.MaterialInstanceDynamic)))
    (:then_1
      (if (Variables|Default|GetisHat)
        (Rendering|Material|SetScalarParameterValue (Variables|Default|GetHatMaterial) "AlphaLength" _alphalength :!class /Script/Engine.MaterialInstanceDynamic)))
    (:then_2
      (if (Variables|Default|GetisAC)
        (Rendering|Material|SetScalarParameterValue (Variables|Default|GetACMaterial) "AlphaLength" _alphalength :!class /Script/Engine.MaterialInstanceDynamic)))
    (:then_3
      (if (Variables|Default|GetisSub)
        (Rendering|Material|SetScalarParameterValue (Variables|Default|GetSubMaterial) "AlphaLength" _alphalength :!class /Script/Engine.MaterialInstanceDynamic)))
    (:then_4
      (if (Variables|Default|GetisSub1)
        (Rendering|Material|SetScalarParameterValue (Variables|Default|GetSub1Material) "AlphaLength" _alphalength :!class /Script/Engine.MaterialInstanceDynamic)))))

(fn GageInit
  (bind _returnvalue (Game|SpawnActorfromClass "/Game/MyGame/Chiga/BP/Particle/BP_GageParticle.BP_GageParticle_C" (Math|Transform|MakeTransform (Transformation|GetWorldLocation (Variables|Default|GetScene)) "0, 0, 0" "2.000000,2.000000,2.000000") "Undefined" 0 0))
  (Variables|Default|SetGage _returnvalue))

(fn GageUpdate
  (bind _gage (Variables|Default|GetGage))
  (Variables|/Game/MyGame/Chiga/BP/Particle/BP_GageParticle.BP_GageParticle_C|SetisSearch _gage (Variables|Default|GetisHit))
  (Transformation|SetActorLocation _gage (Transformation|GetWorldLocation (Variables|Default|GetScene)) false false)
  (Rendering|Material|SetScalarParameterValue (Variables|/Game/MyGame/Chiga/BP/Particle/BP_GageParticle.BP_GageParticle_C|Getmaterial _gage) "Value" (Math|Float|Lerp 1.0 0.35 (/ (Variables|Default|GetSearchRate) 1e+02)) :!class /Script/Engine.MaterialInstanceDynamic)
  (Variables|/Game/MyGame/Chiga/BP/Particle/BP_GageParticle.BP_GageParticle_C|SetScore (Variables|Default|GetGage) (Variables|Default|GetSearchRate)))

(fn SkeletalUpdate
  (bind _returnvalue (Game|Player|GetPlayerPawn 0))
  (bind _skeletalmesh (Variables|Default|GetSkeletalMesh))
  (Utilities|Casting|CastToBP_PlayerHuman _returnvalue
    (:then
      (Rendering|SetVisibility _skeletalmesh false false))
    (:CastFailed
      (Utilities|Casting|CastToBP_PlayerDrone _returnvalue)
      (Rendering|SetVisibility _skeletalmesh true false))))

(fn DestroyUI
  (CallFunction|DestroyValidActor (Variables|Default|GetminimapUI))
  (CallFunction|DestroyValidActor (Variables|Default|GetGage))
  (CallFunction|DestroyValidActor (Variables|Default|GetscanParticle)))

(fn SearchJudgement
  (params (type :type E_NPCType%20Enum :default "NewEnumerator0"))
  (bind _scanparticle (Variables|Default|GetscanParticle))
  (bind _gage (Variables|Default|GetGage))
  (bind _material (Variables|/Game/MyGame/Chiga/BP/Particle/BP_GageParticle.BP_GageParticle_C|Getmaterial _gage))
  (if (not (Variables|Default|GetisDirectSearched))
    (if (not (Variables|Default|GetisJugment))
      (switch Utilities|FlowControl|Switch|SwitchonE_NPCType type
        (:NewEnumerator0
          (LocalVariables|Setspawn "/Game/MyGame/Chiga/BP/Particle/BP_ParticleSafe.BP_ParticleSafe_C")
          (bind _output_get (LocalVariables|SetColor "(R=0.000000,G=0.736171,B=5.000000,A=1.000000)"))
          (LocalVariables|SetScanColor _output_get))
        (:NewEnumerator1
          (LocalVariables|Setspawn "/Game/MyGame/Chiga/BP/Particle/BP_ParticleDenger.BP_ParticleDenger_C" :!label _label)
          (LocalVariables|SetColor "(R=5.000000,G=0.000000,B=1.700821,A=1.000000)")
          (LocalVariables|SetScanColor "(R=5.000000,G=0.000000,B=0.000000,A=1.000000)"))
        (:NewEnumerator2
          (goto _label)))
      (bind _returnvalue (Game|SpawnActorfromClass (LocalVariables|Getspawn) (Math|Transform|MakeTransform "0, 0, 0" "0, 0, 0" "1,1,1") "Undefined" 0 0))
      (bind _asbp_base_particle (Utilities|Casting|CastToBP_BaseParticle _returnvalue))
      (Default|SetActor _asbp_base_particle self)
      (Actor|SetLifeSpan _asbp_base_particle 3.0)
      (Rendering|Material|SetVectorParameterValue _material "ColorEm" (LocalVariables|GetColor) :!class /Script/Engine.MaterialInstanceDynamic)
      (Rendering|Material|SetVectorParameterValue _material "Color" (LocalVariables|GetScanColor) :!class /Script/Engine.MaterialInstanceDynamic)
      (if (Utilities|IsValid _scanparticle)
        _
        (else
          (CallFunction|CreateParticle)))
      (for _array_element (Variables|/Game/MyGame/Chiga/BP/Particle/BP_ParticleBase.BP_ParticleBase_C|Getmaterial _scanparticle)
        (Rendering|Material|SetVectorParameterValue _array_element "Color" (LocalVariables|GetScanColor) :!class /Script/Engine.MaterialInstanceDynamic))
      (for _array_element_2 (Variables|Default|Getmaterial)
        (Rendering|Material|SetVectorParameterValue _array_element_2 "NPCColor" (LocalVariables|GetColor) :!class /Script/Engine.MaterialInstanceDynamic)
        (Variables|Default|SetisDirectSearched true)))))

(fn MaterialInit
  (bind _mesh (Variables|Character|GetMesh))
  (bind _mesh_2 (Variables|Character|GetMesh))
  (bind _glass (Variables|Default|GetGlass))
  (bind _hat (Variables|Default|GetHat))
  (bind _ac (Variables|Default|GetAC))
  (bind _sub (Variables|Default|GetSub))
  (bind _sub2 (Variables|Default|GetSub2))
  (bind _sm_hair (Variables|Default|GetSM_Hair))
  (CallFunction|NPCRandomHair (Variables|Default|GetSM_Hair))
  (Utilities|FlowControl|Sequence
    (:then_0
      (bind _returnvalue (Rendering|Material|CreateDynamicMaterialInstance _mesh_2 0 "/Game/MyGame/Chiga/Material/NPC/NPC_Face/M_Face_Inst.M_Face_Inst" "None" :!class /Script/Engine.PrimitiveComponent))
      (Rendering|Material|SetMaterial _mesh_2 0 _returnvalue)
      (bind _randomnum (CallFunction|NPCRandomTextureFace _returnvalue))
      (Utilities|Array|Add (Variables|Default|Getmaterials) _returnvalue)
      (bind _ismaterial (CallFunction|NPCRandomGlass _randomnum (Variables|Default|GetGlass)))
      (Variables|Default|SetisGlass _ismaterial)
      (bind _returnvalue_2 (Rendering|Material|CreateDynamicMaterialInstance _mesh 1 "/Game/MyGame/Chiga/Material/NPC/NPC_Face/M_Body_Inst.M_Body_Inst" "None" :!class /Script/Engine.PrimitiveComponent))
      (Rendering|Material|SetMaterial _mesh 1 _returnvalue_2)
      (CallFunction|NPCRandomTextureBody _returnvalue_2)
      (Utilities|Array|Add (Variables|Default|Getmaterials) _returnvalue_2)
      (bind _ismaterial_2 (CallFunction|NPCRandomHat (Variables|Default|GetHat)))
      (Variables|Default|SetisHat _ismaterial_2)
      (Utilities|FlowControl|Sequence
        (:then_0
          (if (not (Variables|Default|GetisHat))
            (bind _ismaterial_3 (CallFunction|NPCRandomAC (Variables|Default|GetAC)))
            (Variables|Default|SetisAC _ismaterial_3)))
        (:then_1
          (if (not (Variables|Default|GetisHat))
            (bind _ismaterial_4 (CallFunction|NPCRandomSub1 (Variables|Default|GetSub)))
            (Variables|Default|SetisSub _ismaterial_4)))
        (:then_2
          (bind _ismaterial_5 (CallFunction|NPCRandomSub2 (Variables|Default|GetSub2)))
          (Variables|Default|SetisSub1 _ismaterial_5))))
    (:then_1
      (bind _returnvalue_3 (Rendering|Material|CreateDynamicMaterialInstance _sm_hair 0 "/Game/MyGame/Models/Character/NPC/M_Hair_Inst.M_Hair_Inst" "None" :!class /Script/Engine.PrimitiveComponent))
      (Rendering|Material|SetMaterial _sm_hair 0 _returnvalue_3)
      (bind _output_get (Variables|Default|SethairMaterial _returnvalue_3))
      (|ChangeCOlorHair _output_get))
    (:then_2
      (if (Variables|Default|GetisGlass)
        (bind _returnvalue_4 (Rendering|Material|CreateDynamicMaterialInstance _glass 0 "/Game/MyGame/Chiga/Material/NPC/NPC_AC/M_NPCGlass_Inst.M_NPCGlass_Inst" "None" :!class /Script/Engine.PrimitiveComponent))
        (Rendering|Material|SetMaterial _glass 0 _returnvalue_4)
        (bind _output_get_2 (Variables|Default|SetGlassMaterial _returnvalue_4))
        (|ChangeCOlorHair_2 _output_get_2)))
    (:then_3
      (if (Variables|Default|GetisHat)
        (bind _returnvalue_5 (Rendering|Material|CreateDynamicMaterialInstance _hat 0 "/Game/MyGame/Chiga/Material/NPC/NPC_AC/M_NPCHat_Inst.M_NPCHat_Inst" "None" :!class /Script/Engine.PrimitiveComponent))
        (Rendering|Material|SetMaterial _hat 0 _returnvalue_5)
        (bind _output_get_3 (Variables|Default|SetHatMaterial _returnvalue_5))
        (|ChangeCOlorHair_2_2 _output_get_3)))
    (:then_4
      (if (Variables|Default|GetisAC)
        (bind _returnvalue_6 (Rendering|Material|CreateDynamicMaterialInstance _ac 0 "/Game/MyGame/Chiga/Material/NPC/NPC_AC/M_NPCAC_Inst.M_NPCAC_Inst" "None" :!class /Script/Engine.PrimitiveComponent))
        (Rendering|Material|SetMaterial _ac 0 _returnvalue_6)
        (bind _output_get_4 (Variables|Default|SetACMaterial _returnvalue_6))
        (|ChangeCOlorHair_2_3 _output_get_4)))
    (:then_5
      (if (Variables|Default|GetisSub)
        (bind _returnvalue_7 (Rendering|Material|CreateDynamicMaterialInstance _sub 0 "/Game/MyGame/Chiga/Material/NPC/NPC_AC/M_NPCSubNoHat_Inst.M_NPCSubNoHat_Inst" "None" :!class /Script/Engine.PrimitiveComponent))
        (Rendering|Material|SetMaterial _sub 0 _returnvalue_7)
        (bind _output_get_5 (Variables|Default|SetSubMaterial _returnvalue_7))
        (|ChangeCOlorHair_2_4 _output_get_5)))
    (:then_6
      (if (Variables|Default|GetisSub1)
        (bind _returnvalue_8 (Rendering|Material|CreateDynamicMaterialInstance _sub2 0 "/Game/MyGame/Chiga/Material/NPC/NPC_AC/M_NPCSub_Inst.M_NPCSub_Inst" "None" :!class /Script/Engine.PrimitiveComponent))
        (Rendering|Material|SetMaterial _sub2 0 _returnvalue_8)
        (bind _output_get_6 (Variables|Default|SetSub1Material _returnvalue_8))
        (|ChangeCOlorHair_2_4_2 _output_get_6)))))

(fn TextureSet
  (params (material :type Material%20Instance%20Dynamic%20Object%20Reference) (Base :type Texture%20Object%20Reference) (Rafnes :type Texture%20Object%20Reference) (Normal :type Texture%20Object%20Reference))
  (Rendering|Material|SetTextureParameterValue material "Body_Color" Base)
  (Rendering|Material|SetTextureParameterValue material "Body_Rafnes" Rafnes)
  (Rendering|Material|SetTextureParameterValue material "Body_Normal" Normal))