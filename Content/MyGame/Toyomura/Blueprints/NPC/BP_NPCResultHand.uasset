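; NPC actor, apparently for a result scene, that rebuilds a saved appearance and can be lit by an orange spotlight.
; MaterialLoad removes SkeletalMesh, then applies data IDs to hair, face, body and optional glasses, hat, sub-hair and accessory parts through dynamic material instances.
; Tick watches SpotChange: when true it spawns the spotlight via a DoOnce, when false it fades intensity by a countdown and destroys the light.
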(event EventBeginPlay)

(event EventDestroyed)

(event EventTick
  (params (DeltaSeconds :type Float%20%28single-precision%29))
  (bind _spotlight (Variables|Default|GetSpotLight))
  (Variables|Default|SetdeltaTime DeltaSeconds)
  (if (Variables|Default|GetSpotChange)
    (if (not (Utilities|IsValid (Variables|Default|GetSpotLight)))
      (Utilities|FlowControl|DoOnce false
        (:Completed
          (CallFunction|SpotON))))
    (elif (Utilities|IsValid _spotlight)
      (bind _output_get (Variables|Default|SetTime (Math|Float|Clamp(Float) (- (Variables|Default|GetTime) (Variables|Default|GetdeltaTime)))))
      (Rendering|Components|Light|SetIntensity _spotlight (Math|Float|Lerp 0.0 (Variables|Default|GetSpotPower) (Math|Float|Clamp(Float) (- (Variables|Default|GetTime) (Variables|Default|GetdeltaTime)))))
      (if (<= _output_get 0.0)
        (CallFunction|SpotOFF)))))

(fn ConstructionScript)

(fn MaterialLoad
  (params (Data :type ST%20Save%20NPC%20Data%20Structure))
  (bind _data (Utilities|Struct|BreakST_SaveNPCData Data))
  (bind _mesh (Variables|Character|GetMesh))
  (bind _mesh_2 (Variables|Character|GetMesh))
  (bind _glass (Variables|Default|GetGlass))
  (bind _hat (Variables|Default|GetHat))
  (bind _ac (Variables|Default|GetAC))
  (bind _sm_hair (Variables|Default|GetSM_Hair))
  (bind _sub (Variables|Default|GetSub))
  (bind _sub2 (Variables|Default|GetSub2))
  (bind (_hairid _faceid _haircolorid _bodyid _glassid _glassuse _hatid _hatuse _acid _acuse _subid _subuse _sub2id _sub2use _glasscolorid _hatcolorid _accolorid _subcolorid _sub2colorid) (Utilities|Struct|BreakST_NPCData _data))
  (Components|DestroyComponent (Variables|Default|GetSkeletalMesh))
  (LocalVariables|SetNPCData "")
  (Utilities|FlowControl|Sequence
    (:then_0
      ;[1 1 1] 髪の毛
      (CallFunction|NPCHair (Variables|Default|GetSM_Hair) _hairid)
      (bind _returnvalue (Rendering|Material|CreateDynamicMaterialInstance _sm_hair 0 "/Game/MyGame/Models/Character/NPC/M_Hair_Inst.M_Hair_Inst" "None" :!class /Script/Engine.PrimitiveComponent))
      (Rendering|Material|SetMaterial _sm_hair 0 _returnvalue)
      (bind _output_get (Variables|Default|SethairMaterial _returnvalue))
      (CallFunction|NPCRandomTextureHair _output_get false _haircolorid))
    (:then_1
      ;[1 1 1] 顔
      (bind _returnvalue_2 (Rendering|Material|CreateDynamicMaterialInstance _mesh_2 0 "/Game/MyGame/Chiga/Material/NPC/NPC_Face/M_Face_Inst.M_Face_Inst" "None" :!class /Script/Engine.PrimitiveComponent))
      (Rendering|Material|SetMaterial _mesh_2 0 _returnvalue_2)
      (CallFunction|NPCTextureFace _returnvalue_2 _faceid))
    (:then_2
      ;[1 1 1] 眼鏡
      (if _glassuse
        (CallFunction|NPCGlass _faceid (Variables|Default|GetGlass) _glassid)
        (bind _returnvalue_3 (Rendering|Material|CreateDynamicMaterialInstance _glass 0 "/Game/MyGame/Chiga/Material/NPC/NPC_AC/M_NPCGlass_Inst.M_NPCGlass_Inst" "None" :!class /Script/Engine.PrimitiveComponent))
        (Rendering|Material|SetMaterial _glass 0 _returnvalue_3)
        (bind _output_get_2 (Variables|Default|SetGlassMaterial _returnvalue_3))
        (CallFunction|NPCGlassTexture _output_get_2 _glasscolorid)))
    (:then_3
      ;[1 1 1] 体
      (bind _returnvalue_4 (Rendering|Material|CreateDynamicMaterialInstance _mesh 1 "/Game/MyGame/Chiga/Material/NPC/NPC_Face/M_Body_Inst.M_Body_Inst" "None" :!class /Script/Engine.PrimitiveComponent))
      (Rendering|Material|SetMaterial _mesh 1 _returnvalue_4)
      (CallFunction|NPCTextureBody _returnvalue_4 _bodyid))
    (:then_4
      ;[1 1 1] 帽子
      (if _hatuse
        (CallFunction|NPCHat (Variables|Default|GetHat) _hatid)
        (bind _returnvalue_5 (Rendering|Material|CreateDynamicMaterialInstance _hat 0 "/Game/MyGame/Chiga/Material/NPC/NPC_AC/M_NPCHat_Inst.M_NPCHat_Inst" "None" :!class /Script/Engine.PrimitiveComponent))
        (Rendering|Material|SetMaterial _hat 0 _returnvalue_5)
        (bind _output_get_3 (Variables|Default|SetHatMaterial _returnvalue_5))
        (CallFunction|NPCHatTexture _output_get_3 _hatcolorid)))
    (:then_5
      ;[1 1 1] サブ髪型1
      (if _subuse
        (CallFunction|NPCSub1 (Variables|Default|GetSub) _subid)
        (bind _returnvalue_6 (Rendering|Material|CreateDynamicMaterialInstance _sub 0 "/Game/MyGame/Chiga/Material/NPC/NPC_AC/M_NPCSubNoHat_Inst.M_NPCSubNoHat_Inst" "None" :!class /Script/Engine.PrimitiveComponent))
        (Rendering|Material|SetMaterial _sub 0 _returnvalue_6)
        (bind _output_get_4 (Variables|Default|SetSubMaterial _returnvalue_6))
        (CallFunction|NPCRandomTextureHair _output_get_4 false _subcolorid)))
    (:then_6
      ;[1 1 1] サブ髪型2
      (if _sub2use
        (CallFunction|NPCSub2 _sub2 _sub2id)
        (bind _returnvalue_7 (Rendering|Material|CreateDynamicMaterialInstance _sub2 0 "/Game/MyGame/Chiga/Material/NPC/NPC_AC/M_NPCSubNoHat_Inst.M_NPCSubNoHat_Inst" "None" :!class /Script/Engine.PrimitiveComponent))
        (Rendering|Material|SetMaterial _sub2 0 _returnvalue_7)
        (bind _output_get_5 (Variables|Default|SetSub1Material _returnvalue_7))
        (CallFunction|NPCRandomTextureHair _output_get_5 false _sub2colorid)))
    (:then_7
      ;[1 1 1] アクセサリ
      (if _acuse
        (CallFunction|NPCAC (Variables|Default|GetAC) _acid)
        (bind _returnvalue_8 (Rendering|Material|CreateDynamicMaterialInstance _ac 0 "/Game/MyGame/Chiga/Material/NPC/NPC_AC/M_NPCAC_Inst.M_NPCAC_Inst" "None" :!class /Script/Engine.PrimitiveComponent))
        (Rendering|Material|SetMaterial _ac 0 _returnvalue_8)
        (bind _output_get_6 (Variables|Default|SetACMaterial _returnvalue_8))
        (CallFunction|NPCACTexture _output_get_6 _accolorid)))))

(fn SpotON
  (bind _returnvalue (AddComponent|AddSpotLightComponent false))
  (bind _output_get (Variables|Default|SetSpotLight _returnvalue))
  (Transformation|SetRelativeLocation _output_get (Variables|/Script/Engine.SceneComponent|GetRelativeLocation (Variables|Default|GetSpotScene)) false false)
  (Transformation|SetRelativeRotation _output_get "-90.000000,180.000000,540.000000" false false)
  (Rendering|Components|Light|SetIntensity _output_get (Variables|Default|GetSpotPower))
  (Rendering|Components|Light|SetLightColor _output_get "(R=0.733333,G=0.251404,B=0.000000,A=1.000000)" true))

(fn SpotOFF
  (Components|DestroyComponent (Variables|Default|GetSpotLight)))