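; Smuggler NPC that meets a partner, negotiates, then leaves the field.
; Once a timer elapses on Tick, it sets the Smuggle flag on its detour crowd AI controller, unless flagged as SmugglePartner, and restarts the brain logic.
; When both controllers report arrival, it smoothly turns toward the partner and negotiates for 20 seconds before setting LeaveTheField and restarting logic.
; CheckOn blocks the start, turning and departure.
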(event Custom|Negotiations
  (bind _detourcrowdaicontroller (Variables|Default|GetDetourCrowdAIController))
  ;[1 1 1] 交渉中
  (Variables|Default|SetIsNegotiations true)
  (Utilities|FlowControl|Delay 2e+01)
  (if (not (Variables|Default|GetCheckOn))
    (Variables|Default|SetIsNegotiations false)
    (Variables|/Game/MyGame/Takanashi/BluePrint/BP_DetourCrowdAIController.BP_DetourCrowdAIController_C|SetSmuggle _detourcrowdaicontroller false)
    (Variables|/Game/MyGame/Takanashi/BluePrint/BP_DetourCrowdAIController.BP_DetourCrowdAIController_C|SetArrival _detourcrowdaicontroller false)
    (Variables|/Game/MyGame/Takanashi/BluePrint/BP_DetourCrowdAIController.BP_DetourCrowdAIController_C|SetLeaveTheField _detourcrowdaicontroller true)
    (Class|BrainComponent|RestartLogic (Variables|/Script/AIModule.AIController|GetBrainComponent _detourcrowdaicontroller))))

(event EventBeginPlay
  (|CallParentFunction) ; This node is disabled and will not be called.\nDrag off pins to build functionality.
)

(event Collision|EventActorBeginOverlap
  (params (OtherActor :type Actor%20Object%20Reference))
  (|CallParentFunction OtherActor) ; This node is disabled and will not be called.\nDrag off pins to build functionality.
)

(event EventTick
  (params (DeltaSeconds :type Float%20%28single-precision%29))
  (|CallParentFunction DeltaSeconds)
  (bind _output_get (Variables|Default|SetElapsedTime (+ DeltaSeconds (Variables|Default|GetElapsedTime))))
  (if (>= _output_get (Variables|Default|GetTime))
    (Utilities|FlowControl|Sequence
      (:then_0
        (Utilities|FlowControl|DoOnce false
          (:Completed
            (bind _asbp_detour_crowd_aicontroller (Utilities|Casting|CastToBP_DetourCrowdAIController (AI|GetAIController self)))
            (Variables|Default|SetDetourCrowdAIController _asbp_detour_crowd_aicontroller)
            (if (not (Variables|/Game/MyGame/Takanashi/BluePrint/BP_DetourCrowdAIController.BP_DetourCrowdAIController_C|GetSmugglePartner _asbp_detour_crowd_aicontroller))
              (if (not (Variables|Default|GetCheckOn))
                (if (not (Variables|/Game/MyGame/Takanashi/BluePrint/BP_DetourCrowdAIController.BP_DetourCrowdAIController_C|GetSmuggle _asbp_detour_crowd_aicontroller))
                  (Variables|/Game/MyGame/Takanashi/BluePrint/BP_DetourCrowdAIController.BP_DetourCrowdAIController_C|SetSmuggle _asbp_detour_crowd_aicontroller true)
                  (Class|BrainComponent|RestartLogic (Variables|/Script/AIModule.AIController|GetBrainComponent _asbp_detour_crowd_aicontroller))))))))
      (:then_1
        (if (Variables|/Game/MyGame/Takanashi/BluePrint/BP_DetourCrowdAIController.BP_DetourCrowdAIController_C|GetArrival (Variables|Default|GetDetourCrowdAIController))
          (bind _asbp_detour_crowd_aicontroller_2 (Utilities|Casting|CastToBP_DetourCrowdAIController (AI|GetAIController (Variables|/Game/MyGame/Takanashi/BluePrint/BP_DetourCrowdAIController.BP_DetourCrowdAIController_C|GetSmugglerPartner (Variables|Default|GetDetourCrowdAIController)))))
          (if (Variables|/Game/MyGame/Takanashi/BluePrint/BP_DetourCrowdAIController.BP_DetourCrowdAIController_C|GetArrival _asbp_detour_crowd_aicontroller_2)
            (if (not (Variables|Default|GetCheckOn))
              (Transformation|SetActorRotation (Math|Interpolation|RInterpTo (Transformation|GetActorRotation) (Math|Rotator|MakeRotator 0.0 0.0 (.Yaw (Math|Rotator|BreakRotator (Math|Rotator|FindLookatRotation (Transformation|GetActorLocation) (Transformation|GetActorLocation (Variables|/Game/MyGame/Takanashi/BluePrint/BP_DetourCrowdAIController.BP_DetourCrowdAIController_C|GetSmugglerPartner (Variables|Default|GetDetourCrowdAIController))))))) (Utilities|Time|GetWorldDeltaSeconds) 5.0))
              (Utilities|FlowControl|DoOnce false
                (:Completed
                  (CallFunction|Negotiations))))))))))

(fn ConstructionScript
  (|CallParentFunction))