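; BP_Stalker is a stalker NPC, apparently a criminal variant, that sets its Type on BeginPlay and switches into stalking after a delay.
; Tick accumulates elapsed time until it reaches Time, then a DoOnce makes a single attempt at the switch.
; Unless CheckOn is set, that attempt sets Stalk on its BP_DetourCrowdAIController and restarts the brain component's logic.
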(event EventBeginPlay
  (|CallParentFunction)
  (Variables|Default|Settype "NewEnumerator2"))

(event Collision|EventActorBeginOverlap
  (params (OtherActor :type Actor%20Object%20Reference))
  (|CallParentFunction OtherActor) ; This node is disabled and will not be called.\nDrag off pins to build functionality.
)

(event EventTick
  (params (DeltaSeconds :type Float%20%28single-precision%29))
  (|CallParentFunction DeltaSeconds)
  (bind _output_get (Variables|Default|SetElapsedTime (+ DeltaSeconds (Variables|Default|GetElapsedTime))))
  (if (>= _output_get (Variables|Default|GetTime))
    (Utilities|FlowControl|DoOnce false
      (:Completed
        (bind _asbp_detour_crowd_aicontroller (Utilities|Casting|CastToBP_DetourCrowdAIController (AI|GetAIController self)))
        (if (not (Variables|Default|GetCheckOn))
          (Variables|/Game/MyGame/Takanashi/BluePrint/BP_DetourCrowdAIController.BP_DetourCrowdAIController_C|SetStalk _asbp_detour_crowd_aicontroller true)
          (Class|BrainComponent|RestartLogic (Variables|/Script/AIModule.AIController|GetBrainComponent _asbp_detour_crowd_aicontroller)))))))

(fn ConstructionScript
  (|CallParentFunction))