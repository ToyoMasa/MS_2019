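; Hacker criminal NPC that disrupts the player drone inside its HackingArea.
; A drone entering the area triggers a news alert and, below level 3, gets flagged as hacked and logs the crime once; leaving or destroying the hacker clears the flag.
; After a timed delay, Tick switches its DetourCrowd AI controller to hack mode and restarts its logic unless CheckOn is set.
; MaterialInitNext randomizes hair and applies hacker textures through dynamic materials.
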(event OnComponentBeginOverlap(HackingArea)
  (params (OverlappedComponent :type Primitive%20Component%20Object%20Reference) (OtherActor :type Actor%20Object%20Reference) (OtherComp :type Primitive%20Component%20Object%20Reference) (OtherBodyIndex :type Integer) (bFromSweep :type Boolean) (SweepResult :type Hit%20Result%20Structure%20%28by%20ref%29))
  (bind _asbp_player_drone (Utilities|Casting|CastToBP_PlayerDrone OtherActor))
  (bind _asbp_player_base (Utilities|Casting|CastToBP_PlayerBase (Game|Player|GetPlayerPawn 0)))
  (Default|RecieveNews _asbp_player_base "ハッカーが現れました！")
  (if (not (>= (Variables|/Game/MyGame/Toyomura/Blueprints/Player/BP_PlayerDrone.BP_PlayerDrone_C|GetLevel _asbp_player_drone) 3))
    (Variables|/Game/MyGame/Toyomura/Blueprints/Player/BP_PlayerDrone.BP_PlayerDrone_C|SetIsHacking _asbp_player_drone true)
    (Utilities|FlowControl|DoOnce false
      (:Completed
        (CallFunction|CommittedACrime (Variables|Default|GetScore))))))

(event OnComponentEndOverlap(HackingArea)
  (params (OverlappedComponent :type Primitive%20Component%20Object%20Reference) (OtherActor :type Actor%20Object%20Reference) (OtherComp :type Primitive%20Component%20Object%20Reference) (OtherBodyIndex :type Integer))
  (bind _asbp_player_drone (Utilities|Casting|CastToBP_PlayerDrone OtherActor))
  (Variables|/Game/MyGame/Toyomura/Blueprints/Player/BP_PlayerDrone.BP_PlayerDrone_C|SetIsHacking _asbp_player_drone false))

(event EventBeginPlay
  (Variables|Default|SetisHacker true)
  (|CallParentFunction)
  (bind _outactors (Actor|GetAllActorsOfClass "/Game/MyGame/Toyomura/Blueprints/Player/BP_PlayerDrone.BP_PlayerDrone_C"))
  (Variables|Default|SetDrone (Utilities|Array|Get(acopy) _outactors)))

(event Collision|EventActorBeginOverlap
  (params (OtherActor :type Actor%20Object%20Reference))
  (|CallParentFunction OtherActor) ; This node is disabled and will not be called.\nDrag off pins to build functionality.
)

(event EventTick
  (params (DeltaSeconds :type Float%20%28single-precision%29))
  (|CallParentFunction DeltaSeconds)
  (if (not (Variables|Default|GetisDestroy))
    (bind _output_get (Variables|Default|SetElapsedTime (+ DeltaSeconds (Variables|Default|GetElapsedTime))))
    (if (>= _output_get (Variables|Default|GetTime))
      (Utilities|FlowControl|Sequence
        (:then_0
          (Utilities|FlowControl|DoOnce false
            (:Completed
              (bind _asbp_detour_crowd_aicontroller (Utilities|Casting|CastToBP_DetourCrowdAIController (AI|GetAIController self)))
              (Variables|Default|SetDetourCrowdAIController _asbp_detour_crowd_aicontroller)
              (if (not (Variables|Default|GetCheckOn))
                (Variables|/Game/MyGame/Takanashi/BluePrint/BP_DetourCrowdAIController.BP_DetourCrowdAIController_C|SetHack _asbp_detour_crowd_aicontroller true)
                (Class|BrainComponent|RestartLogic (Variables|/Script/AIModule.AIController|GetBrainComponent _asbp_detour_crowd_aicontroller))))))))))

(event EventMaterialInitNext
  (bind _mesh (Variables|Character|GetMesh))
  (bind _mesh_2 (Variables|Character|GetMesh))
  (bind _sm_hair (Variables|Default|GetSM_Hair))
  (CallFunction|NPCRandomHair (Variables|Default|GetSM_Hair))
  (bind _returnvalue (Rendering|Material|CreateDynamicMaterialInstance _mesh_2 0 "/Game/MyGame/Chiga/Material/NPC/NPC_Face/M_Face_Inst.M_Face_Inst" "None" :!class /Script/Engine.PrimitiveComponent))
  (Rendering|Material|SetMaterial _mesh_2 0 _returnvalue)
  (Rendering|Material|SetTextureParameterValue _returnvalue "Face_Color" "/Game/MyGame/Chiga/Texture/NPC_texture/NPC_face/NPC_face_025_BaseColor.NPC_face_025_BaseColor")
  (Rendering|Material|SetTextureParameterValue _returnvalue "Face_Rafnes" "/Game/MyGame/Chiga/Texture/NPC_texture/NPC_face/NPC_face_025_OcclusionRoughnessMetallic.NPC_face_025_OcclusionRoughnessMetallic")
  (Utilities|Array|Add (Variables|Default|Getmaterials) _returnvalue)
  (bind _returnvalue_2 (Rendering|Material|CreateDynamicMaterialInstance _mesh 1 "/Game/MyGame/Chiga/Material/NPC/NPC_Face/M_Body_Inst.M_Body_Inst" "None" :!class /Script/Engine.PrimitiveComponent))
  (Rendering|Material|SetMaterial _mesh 1 _returnvalue_2)
  (Rendering|Material|SetTextureParameterValue _returnvalue_2 "Body_Color" "/Game/MyGame/Chiga/Material/NPC/NPC_body/NPC_body_046_BaseColor.NPC_body_046_BaseColor")
  (Rendering|Material|SetTextureParameterValue _returnvalue_2 "Body_Rafnes" "/Game/MyGame/Chiga/Material/NPC/NPC_body/NPC_body_046_OcclusionRoughnessMetallic.NPC_body_046_OcclusionRoughnessMetallic")
  (Rendering|Material|SetTextureParameterValue _returnvalue_2 "Body_Normal" "/Game/MyGame/Chiga/Material/NPC/NPC_body/NPC_body_046_Normal.NPC_body_046_Normal")
  (Utilities|Array|Add (Variables|Default|Getmaterials) _returnvalue_2)
  (bind _returnvalue_3 (Rendering|Material|CreateDynamicMaterialInstance _sm_hair 0 "/Game/MyGame/Models/Character/NPC/M_Hair_Inst.M_Hair_Inst" "None" :!class /Script/Engine.PrimitiveComponent))
  (Rendering|Material|SetMaterial _sm_hair 0 _returnvalue_3)
  (Rendering|Material|SetTextureParameterValue _returnvalue_3 "BaseColor" "/Game/MyGame/Chiga/Texture/NPC_texture/NPC_hair_texture/hair_ac_011_BaseColor.hair_ac_011_BaseColor")
  (Rendering|Material|SetTextureParameterValue _returnvalue_3 "BaseColor" "/Game/MyGame/Chiga/Texture/NPC_texture/NPC_hair_texture/hair_ac_011_OcclusionRoughnessMetallic.hair_ac_011_OcclusionRoughnessMetallic")
  (Variables|Default|SethairMaterial _returnvalue_3))

(event EventDestroyed
  (bind _drone (Variables|Default|GetDrone))
  (Variables|/Game/MyGame/Toyomura/Blueprints/Player/BP_PlayerDrone.BP_PlayerDrone_C|SetIsHacking _drone false)
  (Variables|/Game/MyGame/Takanashi/UI/W_TestHacking.W_TestHacking_C|SetType (Variables|/Game/MyGame/Toyomura/Blueprints/Player/BP_PlayerDrone.BP_PlayerDrone_C|GetTestHacking _drone) "NewEnumerator5"))

(fn ConstructionScript
  (|CallParentFunction))