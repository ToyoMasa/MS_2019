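; BP_Thief is a criminal NPC that pickpockets, extending a parent class's crime and search events.
; Once elapsed time passes the criminal start time, optionally overridden by StartTime, it fires once to set Pickpocket on its detour crowd AI controller and restart brain logic, unless CheckOn is set.
; Committing a crime shows the wallet mesh and sends news to the player pawn.
; A search judgement hides the wallet again.
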(event EventBeginPlay
  (bind _starttime (Variables|Default|GetStartTime))
  (Variables|Default|SetCriminalType "NewEnumerator3")
  (|CallParentFunction)
  (Variables|Default|Settype "NewEnumerator2")
  (if (>= _starttime 0.0)
    (Variables|Default|SetCriminalStartTime _starttime)))

(event Collision|EventActorBeginOverlap
  (params (OtherActor :type Actor%20Object%20Reference))
  (|CallParentFunction OtherActor) ; This node is disabled and will not be called.\nDrag off pins to build functionality.
)

(event EventTick
  (params (DeltaSeconds :type Float%20%28single-precision%29))
  (|CallParentFunction DeltaSeconds)
  (bind _output_get (Variables|Default|SetElapsedTime (+ DeltaSeconds (Variables|Default|GetElapsedTime))))
  (if (>= _output_get (Variables|Default|GetCriminalStartTime))
    (Utilities|FlowControl|DoOnce false
      (:Completed
        (bind _asbp_detour_crowd_aicontroller (Utilities|Casting|CastToBP_DetourCrowdAIController (AI|GetAIController self)))
        (if (not (Variables|Default|GetCheckOn))
          (Variables|/Game/MyGame/Takanashi/BluePrint/BP_DetourCrowdAIController.BP_DetourCrowdAIController_C|SetPickpocket _asbp_detour_crowd_aicontroller true)
          (Class|BrainComponent|RestartLogic (Variables|/Script/AIModule.AIController|GetBrainComponent _asbp_detour_crowd_aicontroller)))))))

(event EventCommittedACrime
  (params (Score :type Integer))
  (|CallParentFunction Score)
  (Rendering|SetVisibility (Variables|Default|GetWallet) true false)
  (bind _asbp_player_base (Utilities|Casting|CastToBP_PlayerBase (Game|Player|GetPlayerPawn 0)))
  (Default|ReceiveNews _asbp_player_base 2))

(event EventSearchJudgement
  (params (type :type E_NPCType%20Enum :default "NewEnumerator0"))
  (|CallParentFunction type)
  (Rendering|SetVisibility (Variables|Default|GetWallet) false false))

(fn ConstructionScript
  (|CallParentFunction))