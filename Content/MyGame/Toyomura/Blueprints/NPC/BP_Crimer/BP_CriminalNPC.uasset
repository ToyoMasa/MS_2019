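; Criminal crowd NPC that can be searched and arrested, adding to the game score.
; AIWait stops it, plays surprise and arrest gauge states, awards the arrest score and spawns handcuffs.
; Tick then animates the handcuffs' AlphaLength material parameter, has the Detour crowd controller spawn a replacement NPC at an off-screen point, and destroys this one.
; SearchEnd redefines base logic to bypass the parent's special Denger handling; hologram spawning is disconnected.
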(event EventBeginPlay
  (|CallParentFunction)
  (CallFunction|ChangeType "NewEnumerator2"))

(event Collision|EventActorBeginOverlap
  (params (OtherActor :type Actor%20Object%20Reference))
  (|CallParentFunction OtherActor) ; This node is disabled and will not be called.\nDrag off pins to build functionality.
)

(event EventTick
  (params (DeltaSeconds :type Float%20%28single-precision%29))
  (|CallParentFunction DeltaSeconds)
  (CallFunction|CreateHologram)
  (if (Variables|Default|GetisAlpha)
    (bind _output_get (Variables|Default|SetalphaTime (Math|Float|Clamp(Float) (+ (Variables|Default|GetalphaTime) 0.005556))))
    (bind _output_get_2 (Variables|Default|SetalphaLength (Math|Float|Lerp 3e+02 -1e+02 _output_get)))
    (|HandAlpha_2 _output_get_2)
    (if (>= (Variables|Default|GetalphaTime) 1.0)
      (if (not (Variables|Default|GetisDestroy))
        (Variables|Default|SetisDestroy true)
        (bind _asbp_detour_crowd_aicontroller (Utilities|Casting|CastToBP_DetourCrowdAIController (AI|GetAIController self)))
        (bind _targetpoint (Default|GetRandomTargetPoint _asbp_detour_crowd_aicontroller :!label _label))
        (if (Class|Actor|WasRecentlyRendered _targetpoint 0.1)
          (Utilities|FlowControl|Delay 0.2)
          (goto _label)
          (else
            (Default|SpawnNPC _asbp_detour_crowd_aicontroller _targetpoint)
            (Actor|DestroyActor (Variables|Default|GetHandcuffs))
            (CallFunction|DestroyUI)
            (Actor|DestroyActor)))))))

(event EventSearchDirect
  (Utilities|FlowControl|Sequence
    (:then_0
      (Variables|Default|SetisSearched true))
    (:then_1
      (Actor|SetLifeSpan 8.0))))

(event EventDestroyed
  (CallFunction|DestroyUI))

(event EventSearchJudgement
  (params (type :type E_NPCType%20Enum :default "NewEnumerator0"))
  ;[1 1 1] 逮捕スコアを加算
  (|CallParentFunction type)
  (bind _asgm_my_game (Utilities|Casting|CastToGM_MyGame (Game|GetGameInstance)))
  (Default|ScoreAdd _asgm_my_game (Variables|Default|GetArrestScore)))

(event EventAIWait
  (params (NPC :type Actor%20Object%20Reference))
  (bind _gage (Variables|Default|GetGage))
  (bind _gage_2 (Variables|Default|GetGage))
  (Variables|Default|SetCheckOn true)
  (AI|Navigation|StopMovement (AI|GetAIController NPC))
  (Utilities|FlowControl|Delay 1.0)
  (Variables|/Game/MyGame/Chiga/BP/Particle/BP_GageParticle.BP_GageParticle_C|SetisWhat _gage true)
  (Variables|/Game/MyGame/Chiga/BP/Particle/BP_GageParticle.BP_GageParticle_C|SetWhatType _gage false)
  (Variables|Default|SetIsSurprised true)
  (Utilities|FlowControl|Delay 1.0)
  (Variables|Default|SetIsArrest true)
  (Variables|/Game/MyGame/Chiga/BP/Particle/BP_GageParticle.BP_GageParticle_C|SetisWhat _gage false)
  (Utilities|FlowControl|Delay 2.0)
  (Variables|Default|SetisAlpha true)
  (Rendering|Material|SetTextureParameterValue (Variables|/Game/MyGame/Chiga/BP/Particle/BP_GageParticle.BP_GageParticle_C|Getmaterial _gage_2) "Icon" (Utilities|Select :Index (Variables|Default|Gettype) :NewEnumerator0 "/Game/MyGame/Chiga/Texture/Icon/blue.blue" :NewEnumerator1 "/Game/MyGame/Chiga/Texture/Icon/red.red" :NewEnumerator2 "/Game/MyGame/Chiga/Texture/Icon/red.red"))
  (Variables|/Game/MyGame/Chiga/BP/Particle/BP_GageParticle.BP_GageParticle_C|SetisChange _gage_2 true)
  (CallFunction|SearchJudgement "NewEnumerator2")
  (bind _returnvalue (Game|SpawnActorfromClass "/Game/MyGame/Chiga/BP/Object/BP_Handcuffs.BP_Handcuffs_C" (Math|Transform|MakeTransform (Transformation|GetWorldLocation (Variables|Default|GetSceneHand)) "0, 0, 0" "1,1,1") "Undefined" 0 0))
  (Variables|Default|SetHandcuffs _returnvalue))

(event EventSearchEnd
  (bind _gage (Variables|Default|GetGage))
  ;[1 1 1] 親のDengerの処理が特殊なためBaseの処理を再定義
  (if (not (Variables|Default|GetisSearchEnd))
    (CallFunction|Jugement)
    (Variables|Default|SetisSearchEnd true)
    (Rendering|Material|SetTextureParameterValue (Variables|/Game/MyGame/Chiga/BP/Particle/BP_GageParticle.BP_GageParticle_C|Getmaterial _gage) "Icon" (Utilities|Select :Index (Variables|Default|Gettype) :NewEnumerator0 "/Game/MyGame/Chiga/Texture/Icon/blue.blue" :NewEnumerator1 "/Game/MyGame/Chiga/Texture/Icon/red.red" :NewEnumerator2 "/Game/MyGame/Chiga/Texture/Icon/red.red"))
    (Variables|/Game/MyGame/Chiga/BP/Particle/BP_GageParticle.BP_GageParticle_C|SetisChange _gage true)
    ;;[1 1 1] ACIDの経験値取得
    (Default|GetSearchEXP (Variables|Default|GetGetDrone))))

(fn ConstructionScript
  (|CallParentFunction))

(fn CreateHologram)

(fn AlphaUpdate
  (if (Variables|Default|GetisAlpha)
    (bind _output_get (Variables|Default|SetalphaTime (Math|Float|Clamp(Float) (+ (Variables|Default|GetalphaTime) 0.005556))))
    (bind _output_get_2 (Variables|Default|SetalphaLength (Math|Float|Lerp 3e+02 -1e+02 _output_get)))
    (|HandAlpha _output_get_2)
    (if (>= (Variables|Default|GetalphaTime) 1.0)
      (if (not (Variables|Default|GetisDestroy))
        (Variables|Default|SetisDestroy true)
        (bind _asbp_detour_crowd_aicontroller (Utilities|Casting|CastToBP_DetourCrowdAIController (AI|GetAIController self)))
        (bind _targetpoint (Default|GetRandomTargetPoint _asbp_detour_crowd_aicontroller :!label _label))
        (if (Class|Actor|WasRecentlyRendered _targetpoint 0.1)
          (goto _label)
          (else
            (Default|SpawnNPC _asbp_detour_crowd_aicontroller _targetpoint)
            (Actor|DestroyActor (Variables|Default|GetHandcuffs))
            (CallFunction|DestroyUI)
            (Actor|DestroyActor)))))))

(fn CommittedACrime
  (params (Score :type Integer))
  (bind _returnvalue (Transformation|GetActorLocation))
  (bind _asgm_my_game (Utilities|Casting|CastToGM_MyGame (Game|GetGameInstance)))
  (Default|ScoreAdd _asgm_my_game Score)
  (Development|PrintString "Committed a crime")
  (Game|SpawnActorfromClass "/Game/MyGame/Chiga/BP/Minimap/BP_PointUI_Child.BP_PointUI_Child_C" (Math|Transform|MakeTransform (Math|Vector|MakeVector (.x _returnvalue) (.y _returnvalue) 1e+02) "0, 0, 0" "1,1,1") "Undefined" 0 0))